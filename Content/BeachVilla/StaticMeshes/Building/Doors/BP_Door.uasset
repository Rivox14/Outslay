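; BP_Door is a hinged door that the player character toggles open and closed through the OpenDoor event.
; The event acts only while the player's BP_ThirdPersonCharacter overlaps the Front component.
; It flips the Opened flag, swaps the A and B yaw endpoints, and replays one Timeline from the start.
; The Timeline track drives a Lerp between those endpoints, swinging the static mesh a quarter turn.
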(event `Open Door`
  (if (`PrimitiveComponent.IsOverlappingActor` (`self.Front`) (cast `/Game/ThirdPerson/Blueprints/BP_ThirdPersonCharacter` (`GameplayStatics.GetPlayerCharacter` 0) :!pure true))
    (if (`self.Opened`)
      (set `self.Opened` false)
      (set `self.B` 0.0)
      (set `self.A` -90.0)
      (bind (_direction _newtrack_0) (`Timeline|Timeline` :!via `PlayFromStart` :!label _label)
        (:`Update`
          (`SceneComponent.K2_SetRelativeRotation` (`self.StaticMesh`) (`KismetMathLibrary.MakeRotator` 0.0 0.0 (`KismetMathLibrary.Lerp` (`self.A`) (`self.B`) _newtrack_0)) false false)))
      (else
        (set `self.Opened` true)
        (set `self.B` -90.0)
        (set `self.A` 0.0)
        (goto _label :!via `PlayFromStart`)))))

(fn `UserConstructionScript`)