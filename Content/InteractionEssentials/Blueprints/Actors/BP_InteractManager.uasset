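; Interaction manager actor that tracks registered interaction components and selects which one the player can currently interact with.
; With several registered, Tick flags the one best aligned with camera or pawn facing by dot product, if above a threshold.
; Trigger helpers forward start, update, complete and cancel to the flagged component.
; Any-key input detects the input type and broadcasts key and device changes, with separate logic adjusting mouse cursor visibility.
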(event `self.ReceiveTick`
  (params (DeltaSeconds :type "Float (single-precision)"))
  (bind _output (`|GetArrayItem` (`self.Interactions`)))
  ;[0 0 0] Tick
  (set `self.DeltaX` DeltaSeconds)
  (`|ExecutionSequence`
    (:`then_0`
      (if (`self.HasMultipleInteractions`)
        (`|ExecutionSequence`
          (:`then_0`
            (`self.TickPrintBestInteractionValues` false)
            (`/Engine/EditorBlueprintResources/StandardMacros.IsValid` (`self.FindBestInteraction`)
              (:`Is Valid`
                (for _array_element (`self.Interactions`)
                  (`/Engine/EditorBlueprintResources/StandardMacros.IsValid` _array_element
                    (:`Is Valid`
                      (if (!= _array_element (`self.FindBestInteraction`))
                        (`/Game/InteractionEssentials/Blueprints/Components/InteractionComponent.SetIsDotProduct` _array_element false)))))
                (`/Game/InteractionEssentials/Blueprints/Components/InteractionComponent.SetIsDotProduct` (`self.FindBestInteraction`) true))
              (:`Is Not Valid`
                (for _array_element_2 (`self.Interactions`)
                  (`/Engine/EditorBlueprintResources/StandardMacros.IsValid` _array_element_2
                    (:`Is Valid`
                      (`/Game/InteractionEssentials/Blueprints/Components/InteractionComponent.SetIsDotProduct` _array_element_2 false)))))))
          (:`then_1`
            (goto _label :!via `ResetBoth`)))
        (else
          (`self.OnceBranchWithReset` (`self.HasAnyInteraction`) :!label _label
            (:`true`
              (`/Engine/EditorBlueprintResources/StandardMacros.IsValid` _output
                (:`Is Valid`
                  (`/Game/InteractionEssentials/Blueprints/Components/InteractionComponent.SetIsDotProduct` _output true))))))))
    (:`then_1`
      (if false
        (for _array_element_3 (`self.Interactions`)
          (`/Engine/EditorBlueprintResources/StandardMacros.IsValid` _array_element_3
            (:`Is Valid`
              (`KismetSystemLibrary.PrintString` (`KismetSystemLibrary.GetDisplayName` _array_element_3) true false (struct :`G` 0.66 :`B` 1.0 :`A` 1.0) 0.001))))))))

(event `self.ReceiveBeginPlay`
  ;[0 0 0] Beginplay
  (`self.EnableInput` (`GameplayStatics.GetPlayerController` 0)))

(event `Key|AnyKey` :consume false :overrideparent false
  (params (Key :type "Key Structure"))
  ;[0 0 0] OnAnyKeyPressed
  (:`Pressed`
    (`self.OnKeyPressed` Key))
  (:`Released`
    (`self.OnKeyReleased` Key)))

(event `OnKeyPressed`
  (params (InKey :type "Key Structure" :default "None"))
  ;[0 0 0] OnAnyKeyPressed
  (set `self.InKey` InKey)
  (`|ExecutionSequence`
    (:`then_0`
      (bind (_lastpressed_key _inputtype) (`/Game/InteractionEssentials/Blueprints/Libraries/BP_InputFunctions.FindInputType` (`self.InKey`)))
      (`self.SetInputType` _inputtype))
    (:`then_1`
      (`self.UpdateInputKey` true (`self.InKey`)))))

(event `OnKeyReleased`
  (params (InKey :type "Key Structure" :default "None"))
  ;[0 0 0] OnAnyKeyPressed
  (set `self.InKey` InKey)
  (`self.UpdateInputKey` false (`self.InKey`)))

(event `TrackMouseCursorVisibility` :!signature `self.UpdateInputType`
  (params (InputType :type "/Game/InteractionEssentials/Blueprints/Enums/EInputType Enum" :default "NewEnumerator0"))
  (bind _returnvalue (`GameplayStatics.GetPlayerController` 0))
  ;[0 0 0] Track Mouse Cursor Visibility
  (switch `/Game/InteractionEssentials/Blueprints/Enums/EInputType` InputType
    (:`NewEnumerator0`
      (`|ExecutionSequence`
        (:`then_0`
          (`/Engine/EditorBlueprintResources/StandardMacros.DoOnce` false :!label _label_2
            (:`Completed`
              _)))
        (:`then_1`
          (goto _label_3 :!via `Reset`))))
    (:`NewEnumerator1`
      (`|ExecutionSequence`
        (:`then_0`
          (`/Engine/EditorBlueprintResources/StandardMacros.DoOnce` false :!label _label_3
            (:`Completed`
              _)))
        (:`then_1`
          (goto _label_2 :!via `Reset`)))))
  (if (not (`self.bShowMouse`))
    (if (`|EnumEquality` (`self.InputType`) "NewEnumerator0")
      (`/Engine/EditorBlueprintResources/StandardMacros.DoOnce` false :!label _label_4
        (:`Completed`
          (set `PlayerController.bShowMouseCursor` true _returnvalue)
          (goto _label_5 :!via `Reset`)))
      (else
        (`/Engine/EditorBlueprintResources/StandardMacros.DoOnce` false :!label _label_5
          (:`Completed`
            (set `PlayerController.bShowMouseCursor` false _returnvalue)
            (bind _returnvalue_2 (`GameUserSettings.GetGameUserSettings`))
            (bind (_returnvalue_x _returnvalue_y) (break `IntPoint` (`GameUserSettings.GetDesktopResolution` _returnvalue_2)))
            (`PlayerController.SetMouseLocation` _returnvalue (/ _returnvalue_x 2) (/ _returnvalue_y 2))
            (goto _label_4 :!via `Reset`)))))))

(fn `FindBestInteraction`
  (returns (ReturnValue :type "/Game/InteractionEssentials/Blueprints/Components/InteractionComponent Object Reference") (DotProductThreshold :type "Float (double-precision)") (MaxValue :type "Float (double-precision)"))
  (locals (CurrentInteraction :type "/Game/InteractionEssentials/Blueprints/Components/InteractionComponent Object Reference") (Dots :type "Array of Float (double-precision)"))
  (bind _dotproductthreshold (`self.DotProductThreshold`))
  (bind (_indexofmaxvalue _maxvalue) (`KismetMathLibrary.MaxOfFloatArray` (`local.Dots`)))
  (for _array_element (`self.Interactions`)
    (`/Engine/EditorBlueprintResources/StandardMacros.IsValid` _array_element
      (:`Is Valid`
        (set `local.CurrentInteraction` _array_element)
        (`KismetArrayLibrary.Array_Add` (`local.Dots`) (`KismetMathLibrary.Dot_VectorVector` (`KismetMathLibrary.Normal` (- (`/Game/InteractionEssentials/Blueprints/Components/InteractionComponent.GetSourceLocation` (`local.CurrentInteraction`)) (select `/Game/InteractionEssentials/Blueprints/Enums/EDotProductMethod` (`/Game/InteractionEssentials/Blueprints/Components/InteractionComponent.DotProductMethod` (`local.CurrentInteraction`)) :`NewEnumerator0` (`PlayerCameraManager.GetCameraLocation` (`GameplayStatics.GetPlayerCameraManager` 0)) :`NewEnumerator1` (`self.K2_GetActorLocation` (`GameplayStatics.GetPlayerPawn` 0))))) (`self.GetActorForwardVector` (select `/Game/InteractionEssentials/Blueprints/Enums/EDotProductMethod` (`/Game/InteractionEssentials/Blueprints/Components/InteractionComponent.DotProductMethod` (`local.CurrentInteraction`)) :`NewEnumerator0` (`GameplayStatics.GetPlayerCameraManager` 0) :`NewEnumerator1` (`GameplayStatics.GetPlayerPawn` 0) :!type "Actor Object Reference")))))))
  (if (>= _maxvalue _dotproductthreshold)
    (return (`|GetArrayItem` (`self.Interactions`) _indexofmaxvalue) _dotproductthreshold _maxvalue)
    (else
      (return null _dotproductthreshold _maxvalue))))

(fn `GetCurrentInteraction`
  (returns (ReturnValue :type "/Game/InteractionEssentials/Blueprints/Components/InteractionComponent Object Reference"))
  (locals (Found :type "/Game/InteractionEssentials/Blueprints/Components/InteractionComponent Object Reference"))
  (for _array_element (`self.Interactions`)
    (`/Engine/EditorBlueprintResources/StandardMacros.IsValid` _array_element
      (:`Is Valid`
        (if (`/Game/InteractionEssentials/Blueprints/Components/InteractionComponent.GetIsDotProduct` _array_element)
          (set `local.Found` _array_element)
          (break)))))
  (return (`local.Found`)))

(fn `HasAnyInteraction`
  (returns (ReturnValue :type Boolean))
  (return (> (`KismetArrayLibrary.Array_Length` (`self.Interactions`)) 0)))

(fn `HasMultipleInteractions`
  (returns (ReturnValue :type Boolean))
  (return (> (`KismetArrayLibrary.Array_Length` (`self.Interactions`)) 1)))

(fn `RegisterInteraction`
  (params (InteractionComp :type "/Game/InteractionEssentials/Blueprints/Components/InteractionComponent Object Reference"))
  (if (not (`KismetArrayLibrary.Array_Contains` (`self.Interactions`) InteractionComp))
    (`KismetArrayLibrary.Array_AddUnique` (`self.Interactions`) InteractionComp)))

(fn `SetInputType`
  (params (InputType :type "/Game/InteractionEssentials/Blueprints/Enums/EInputType Enum" :default "NewEnumerator0"))
  (if (`|EnumInequality` (`self.InputType`) InputType)
    (bind _output_get (set `self.InputType` InputType))
    (`self.UpdateInputType` _output_get))
  (return))

(fn `SetShowMouse`
  (params (bShowMouse :type Boolean))
  (set `self.bShowMouse` bShowMouse))

(fn `TickPrintBestInteractionValues`
  (params (Print :type Boolean))
  (bind (_returnvalue _dotproductthreshold _maxvalue) (`self.FindBestInteraction`))
  (if Print
    (`/Engine/EditorBlueprintResources/StandardMacros.IsValid` _returnvalue
      (:`Is Valid`
        (`KismetSystemLibrary.PrintString` (`KismetStringLibrary.Concat_StrStr` "Threshold: " (`KismetStringLibrary.Conv_DoubleToString` _dotproductthreshold)) true false (struct :`R` 1.0 :`G` 0.753423 :`A` 1.0) 0.1)
        (`KismetSystemLibrary.PrintString` (`KismetStringLibrary.Concat_StrStr` "Max Value: " (`KismetStringLibrary.Conv_DoubleToString` _maxvalue)) true false (struct :`R` 1.0 :`G` 0.246969 :`A` 1.0) 0.1)))))

(fn `UnregisterInteraction`
  (params (InteractionComp :type "/Game/InteractionEssentials/Blueprints/Components/InteractionComponent Object Reference"))
  (if (`KismetArrayLibrary.Array_Contains` (`self.Interactions`) InteractionComp)
    (`/Game/InteractionEssentials/Blueprints/Components/InteractionComponent.SetIsDotProduct` InteractionComp false)
    (`KismetArrayLibrary.Array_RemoveItem` (`self.Interactions`) InteractionComp)))

(fn `UserConstructionScript`)