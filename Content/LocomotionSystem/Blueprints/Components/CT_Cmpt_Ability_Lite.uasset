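; Lightweight ability component that provides cooldown gating for abilities in the locomotion system.
; CheckCooldown returns false while cooling down, otherwise starts the cooldown and returns true.
; StartCooldown, when Cooldown is positive, sets a one-shot timer, raises the cooling flag and fires an on-start event with the duration; the timer's end clears the flag.
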(event `StartCooldown`
  (if (> (`self.Cooldown`) 0.0)
    (`KismetSystemLibrary.K2_SetTimerDelegate` (delegate `Event_CooldownFinish`) (`self.Cooldown`))
    (set `self.IsCoolingDown` true)
    (`self.Event_OnStartCooldown` (`self.Cooldown`))))

(event `Event_CooldownFinish`
  (set `self.IsCoolingDown` false))

(fn `Check&Cooldown`
  (returns (ReturnValue :type Boolean))
  (if (not (`self.IsCoolingDown`))
    (`self.StartCooldown`)
    (return true)
    (else
      (return false))))