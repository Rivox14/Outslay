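; Lite abilities manager component in the locomotion system that adds and removes actor-based abilities on its owner by identifier.
; Register rejects duplicate identifiers or classes, then spawns the ability actor, attaches it to the owner and stores it in parallel arrays.
; Unregister looks up the identifier, clears both entries and destroys the actor.
; Both changes are relayed through server-to-multicast events that fire registered or unregistered dispatchers.
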(event `RegisteredAbility_Server`
  (params (Identifier :type Name))
  (`self.RegisteredAbility_Multicast` Identifier))

(event `RegisteredAbility_Multicast`
  (params (Identifier :type Name))
  (`self.Event_OnRegistered` Identifier))

(event `UnregisteredAbility_Server`
  (params (Identifier :type Name))
  (`self.UnregisteredAbility_Multicast` Identifier))

(event `UnregisteredAbility_Multicast`
  (params (Identifier :type Name))
  (`self.Event_OnUnregistered` Identifier))

(fn `GetAbility`
  (params (Identifier :type Name))
  (returns (ReturnValue :type "Actor Object Reference"))
  (bind _returnvalue (`KismetArrayLibrary.Array_Find` (`self.Identifiers`) Identifier))
  (if (> _returnvalue -1)
    (return (`|GetArrayItem` (`self.Abilities`) _returnvalue))
    (else
      (return null))))

(fn `Register`
  (params (Identifier :type Name) (ActorClass :type "Actor Class Reference"))
  (locals (Local_Registered :type Boolean))
  (`|ExecutionSequence`
    (:`then_0`
      (for _array_element (`self.Identifiers`)
        (if (== _array_element (`local.Identifier`))
          (return))))
    (:`then_1`
      (for _array_element_2 (`self.Abilities`)
        (if (== (`GameplayStatics.GetObjectClass` _array_element_2) (`local.ActorClass`))
          (return))))
    (:`then_2`
      (bind _returnvalue (`|SpawnActorFromClass` (`local.ActorClass`) (`KismetMathLibrary.MakeTransform` (0.0 0.0 0.0)) "Undefined" "SelectDefaultAtRuntime" (`self.GetOwner`) null))
      (`Actor.K2_AttachToActor` _returnvalue (`self.GetOwner`) "None" "SnapToTarget" "SnapToTarget" "SnapToTarget" true)
      (`KismetArrayLibrary.Array_Add` (`self.Abilities`) _returnvalue)
      (`KismetArrayLibrary.Array_Add` (`self.Identifiers`) (`local.Identifier`))
      (`self.RegisteredAbility_Server` (`local.Identifier`)))))

(fn `Unregister`
  (params (Identifier :type Name))
  (locals (Local_Index :type Integer :default 0) (Local_Ability :type "Actor Object Reference"))
  (bind _output_get (set `local.Local_Index` (`KismetArrayLibrary.Array_Find` (`self.Identifiers`) (`local.Identifier`))))
  (if (> _output_get -1)
    (set `local.Local_Ability` (`self.GetAbility` (`local.Identifier`)))
    (`KismetArrayLibrary.Array_Remove` (`self.Identifiers`) (`local.Local_Index`))
    (`KismetArrayLibrary.Array_Remove` (`self.Abilities`) (`local.Local_Index`))
    (`Actor.K2_DestroyActor` (`local.Local_Ability`))
    (`self.UnregisteredAbility_Server` (`local.Identifier`))))