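; Lightweight weapon component that tracks magazine and spare ammo and the current accuracy loss.
; Decrement, reload and AddSpareAmmo, which assigns rather than adds, each fire an OnAmmoChanged event; reload overwrites the magazine with the remaining spare when reserves are low.
; Accuracy loss switches between hipfire and aiming values, starting at hipfire on BeginPlay.
; The Character is resolved through the owning actor's owner.
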(event `self.ReceiveBeginPlay`
  (`self.UseHipfireAccuracyLoss`))

(fn `AddSpareAmmo`
  (params (SpareAmmo :type Integer))
  (set `self.SpareAmmo` SpareAmmo)
  (`self.Event_OnAmmoChanged`))

(fn `DecrementAmmo`
  (set `self.MagazineAmmo` (+ -1 (`self.MagazineAmmo`)))
  (`self.Event_OnAmmoChanged`))

(fn `GetCharacter`
  (returns (Character :type "Character Object Reference"))
  (bind _ascharacter (cast `Character` (`Actor.GetOwner` (`self.GetOwner`))))
  (return _ascharacter))

(fn `isMagazineEmpty`
  (returns (ReturnValue :type Boolean))
  (return (<= (`self.MagazineAmmo`) 0)))

(fn `ReloadAmmo`
  (if (> (`self.SpareAmmo`) (`self.MagazineSize`))
    (set `self.SpareAmmo` (- (+ (`self.SpareAmmo`) (`self.MagazineAmmo`)) (`self.MagazineSize`)))
    (set `self.MagazineAmmo` (`self.MagazineSize`))
    (else
      (set `self.MagazineAmmo` (`self.SpareAmmo`))
      (set `self.SpareAmmo` 0)))
  (`self.Event_OnAmmoChanged`))

(fn `UseAimingAccuracyLoss`
  (set `self.AccuracyLoss` (`self.AimingAccuracyLoss`)))

(fn `UseHipfireAccuracyLoss`
  (set `self.AccuracyLoss` (`self.HipfireAccuracyLoss`)))