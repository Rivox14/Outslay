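; Anim notify state that runs melee weapon hit detection during an attack animation, on authority only.
; Each tick sphere-traces between the current quick-bar weapon's start and end sockets, plus straight and diagonal traces to the previous tick's positions to cover the swept area.
; Hits fire MeleeTraced on the weapon's montage component, once per actor display name.
; Stored positions and hit names clear when the notify ends.
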(fn `CanAttack?`
  (params (Actor :type "Actor Object Reference"))
  (returns (Result :type Boolean))
  (bind _returnvalue (`KismetSystemLibrary.GetDisplayName` Actor))
  (bind _attackmap (`self.AttackMap`))
  (`/Engine/EditorBlueprintResources/StandardMacros.IsValid` Actor
    (:`Is Valid`
      (if (`BlueprintMapLibrary.Map_Contains` _attackmap _returnvalue)
        (return false)
        (else
          (`BlueprintMapLibrary.Map_Add` _attackmap _returnvalue true)
          (return true))))
    (:`Is Not Valid`
      (return false))))

(fn `GetTraceLocation`
  (params (Owner :type "Actor Object Reference"))
  (returns (Start :type "Vector Structure") (End :type "Vector Structure"))
  (locals (Local_Cmpt_Weapon :type "/Game/LocomotionSystem/Blueprints/Components/CT_Cmpt_Weapon_Lite Object Reference") (Local_WeaponActor :type "Actor Object Reference"))
  (bind _returnvalue (`Actor.GetComponentByClass` Owner "/Game/LocomotionSystem/Blueprints/Components/CT_Cmpt_QuickBar_Lite.CT_Cmpt_QuickBar_Lite_C"))
  (bind _local_cmpt_weapon (`local.Local_Cmpt_Weapon`))
  (bind _returnvalue_2 (`Actor.GetComponentByClass` (`local.Local_WeaponActor`) "/Script/Engine.MeshComponent"))
  (`/Engine/EditorBlueprintResources/StandardMacros.IsValid` _returnvalue
    (:`Is Valid`
      (bind _output_get (set `local.Local_WeaponActor` (`/Game/LocomotionSystem/Blueprints/Components/CT_Cmpt_QuickBar_Lite.GetCurrentSlot` _returnvalue)))
      (`/Engine/EditorBlueprintResources/StandardMacros.IsValid` _output_get
        (:`Is Valid`
          (bind _output_get_2 (set `local.Local_Cmpt_Weapon` (`Actor.GetComponentByClass` (`local.Local_WeaponActor`) "/Game/LocomotionSystem/Blueprints/Components/CT_Cmpt_Weapon_Lite.CT_Cmpt_Weapon_Lite_C")))
          (`/Engine/EditorBlueprintResources/StandardMacros.IsValid` _output_get_2
            (:`Is Valid`
              (`/Engine/EditorBlueprintResources/StandardMacros.IsValid` _returnvalue_2
                (:`Is Valid`
                  (return (`SceneComponent.GetSocketLocation` _returnvalue_2 (`/Game/LocomotionSystem/Blueprints/Components/CT_Cmpt_Weapon_Lite.MeleeTraceSocket_Start` _local_cmpt_weapon)) (`SceneComponent.GetSocketLocation` _returnvalue_2 (`/Game/LocomotionSystem/Blueprints/Components/CT_Cmpt_Weapon_Lite.MeleeTraceSocket_End` _local_cmpt_weapon))))))))))))

(fn `Received_NotifyBegin`
  (params (MeshComp :type "SkeletalMeshComponent Object Reference") (Animation :type "AnimSequenceBase Object Reference") (TotalDuration :type "Float (single-precision)") (EventReference :type "AnimNotifyEventReference Structure (by ref)"))
  (returns (ReturnValue :type Boolean))
  (return false))

(fn `Received_NotifyEnd`
  (params (MeshComp :type "SkeletalMeshComponent Object Reference") (Animation :type "AnimSequenceBase Object Reference") (EventReference :type "AnimNotifyEventReference Structure (by ref)"))
  (returns (ReturnValue :type Boolean))
  (`BlueprintMapLibrary.Map_Clear` (`self.AttackMap`))
  (`KismetArrayLibrary.Array_Clear` (`self.TraceStartLocations`))
  (`KismetArrayLibrary.Array_Clear` (`self.TraceEndLocations`))
  (return false))

(fn `Received_NotifyTick`
  (params (MeshComp :type "SkeletalMeshComponent Object Reference") (Animation :type "AnimSequenceBase Object Reference") (FrameDeltaTime :type "Float (single-precision)") (EventReference :type "AnimNotifyEventReference Structure (by ref)"))
  (returns (ReturnValue :type Boolean))
  (locals (LStartLocation :type "Vector Structure") (LEndLocation :type "Vector Structure") (LVLength :type Integer :default 0))
  (bind (_start _end) (`self.GetTraceLocation` (`ActorComponent.GetOwner` (`local.MeshComp`))))
  (if (`Actor.HasAuthority` (`ActorComponent.GetOwner` MeshComp))
    (`|ExecutionSequence`
      (:`then_0`
        (set `local.LStartLocation` _start)
        (set `local.LEndLocation` _end)
        (`self.Trace` (`local.MeshComp`) (`local.LStartLocation`) (`local.LEndLocation`)))
      (:`then_1`
        (bind _output_get (set `local.LVLength` (- (`KismetArrayLibrary.Array_Length` (`self.TraceStartLocations`)) 1)))
        (if (>= _output_get 0)
          (`self.Trace` (`local.MeshComp`) (`|GetArrayItem` (`self.TraceStartLocations`) (`local.LVLength`)) (`local.LStartLocation`))
          (`self.Trace` (`local.MeshComp`) (`|GetArrayItem` (`self.TraceEndLocations`) (`local.LVLength`)) (`local.LEndLocation`))
          (`self.Trace` (`local.MeshComp`) (`|GetArrayItem` (`self.TraceEndLocations`) (`local.LVLength`)) (`local.LStartLocation`))
          (`self.Trace` (`local.MeshComp`) (`|GetArrayItem` (`self.TraceStartLocations`) (`local.LVLength`)) (`local.LEndLocation`))))
      (:`then_2`
        (`KismetArrayLibrary.Array_Add` (`self.TraceStartLocations`) (`local.LStartLocation`))
        (`KismetArrayLibrary.Array_Add` (`self.TraceEndLocations`) (`local.LEndLocation`))
        (return false)))))

(fn `Trace`
  (params (MeshComp :type "SkeletalMeshComponent Object Reference") (TStartLocation :type "Vector Structure") (TEndLocation :type "Vector Structure"))
  (bind _returnvalue (`ActorComponent.GetOwner` MeshComp))
  (bind (_outhit _returnvalue_2) (`KismetSystemLibrary.SphereTraceSingle` MeshComp (`local.TStartLocation`) (`local.TEndLocation`) 15.0 "TraceTypeQuery3" false (`|MakeArray` _returnvalue)))
  (if _returnvalue_2
    (if (`self.CanAttack?` (`.HitActor` (`GameplayStatics.BreakHitResult` _outhit)))
      (`/Game/LocomotionSystem/Blueprints/Components/CT_Cmpt_Montage_Lite.Event_MeleeTraced` (`Actor.GetComponentByClass` (`/Game/LocomotionSystem/Blueprints/Components/CT_Cmpt_QuickBar_Lite.GetCurrentSlot` (`Actor.GetComponentByClass` _returnvalue "/Game/LocomotionSystem/Blueprints/Components/CT_Cmpt_QuickBar_Lite.CT_Cmpt_QuickBar_Lite_C")) "/Game/LocomotionSystem/Blueprints/Components/CT_Cmpt_Montage_Lite.CT_Cmpt_Montage_Lite_C") _outhit))))