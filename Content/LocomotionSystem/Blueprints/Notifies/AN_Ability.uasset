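; Anim notify that forwards a named notify from an animation to one of the owning actor's abilities.
; On firing, it looks up the owner's lite abilities manager component and fetches the ability matching AbilityName.
; It then calls CallEventOnNotify with NotifyName on that ability's lite montage component, guarding each lookup with a validity check.
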(fn `Received_Notify`
  (params (MeshComp :type "SkeletalMeshComponent Object Reference") (Animation :type "AnimSequenceBase Object Reference") (EventReference :type "AnimNotifyEventReference Structure (by ref)"))
  (returns (ReturnValue :type Boolean))
  (bind _returnvalue (`Actor.GetComponentByClass` (`ActorComponent.GetOwner` MeshComp) "/Game/LocomotionSystem/Blueprints/Components/CT_Cmpt_AbilitiesManager_Lite.CT_Cmpt_AbilitiesManager_Lite_C"))
  (bind _returnvalue_2 (`/Game/LocomotionSystem/Blueprints/Components/CT_Cmpt_AbilitiesManager_Lite.GetAbility` _returnvalue (`self.AbilityName`)))
  (bind _returnvalue_3 (`Actor.GetComponentByClass` _returnvalue_2 "/Game/LocomotionSystem/Blueprints/Components/CT_Cmpt_Montage_Lite.CT_Cmpt_Montage_Lite_C"))
  (`/Engine/EditorBlueprintResources/StandardMacros.IsValid` _returnvalue
    (:`Is Valid`
      (`/Engine/EditorBlueprintResources/StandardMacros.IsValid` _returnvalue_2
        (:`Is Valid`
          (`/Engine/EditorBlueprintResources/StandardMacros.IsValid` _returnvalue_3
            (:`Is Valid`
              (`/Game/LocomotionSystem/Blueprints/Components/CT_Cmpt_Montage_Lite.Event_OnNotify` _returnvalue_3 (`self.NotifyName`))
              (return true))))))))