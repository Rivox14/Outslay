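; Behavior tree task that picks a random roam location for the AI pawn and writes it to the MoveToLocation blackboard key.
; Walking pawns get a reachable navmesh point within Radius, and the task fails if none is found.
; Flying pawns get a random altitude and reuse that XY search, falling back to the cached nearest NavMeshBoundsVolume location.
; GetNavMeshLocation and the farthest-sample GetFlightRandomLocation are defined but never called here.
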(event `self.ReceiveExecuteAI`
  (params (OwnerController :type "AIController Object Reference") (ControlledPawn :type "Pawn Object Reference"))
  (bind (_randomlocation _returnvalue) (`self.GetRandomLocation` ControlledPawn))
  (`/Engine/EditorBlueprintResources/StandardMacros.IsValid` ControlledPawn
    (:`Is Valid`
      (if _returnvalue
        (set `self.Location` _randomlocation)
        (`BTFunctionLibrary.SetBlackboardValueAsVector` (`self.MoveToLocation`) (`self.Location`))
        (`self.FinishExecute` true)
        (else
          (`self.FinishExecute` false))))))

(fn `GetFlightRandomLocation`
  (params (Pawn :type "Actor Object Reference"))
  (returns (Location :type "Vector Structure"))
  (locals (CacheVector :type "Array of Vector Structure") (CacheDistance :type "Array of Float (double-precision)"))
  (bind _returnvalue (`Actor.K2_GetActorLocation` Pawn))
  (bind (_randomlocation _returnvalue_2) (`NavigationSystemV1.K2_GetRandomReachablePointInRadius` _returnvalue (`self.Radius`) null null))
  (bind (_output_x _output_y) (`KismetMathLibrary.BreakVector` (`|GetArrayItem` (`local.CacheVector`) (`KismetMathLibrary.MaxOfFloatArray` (`local.CacheDistance`)))))
  (if _returnvalue_2
    (for _ (range 11)
      (`KismetArrayLibrary.Array_Add` (`local.CacheVector`) _randomlocation)
      (`KismetArrayLibrary.Array_Add` (`local.CacheDistance`) (`KismetMathLibrary.Vector_Distance` _returnvalue _randomlocation)))
    (return (`KismetMathLibrary.MakeVector` _output_x _output_y (`KismetMathLibrary.RandomFloatInRange` 300.0 1500.0)))
    (else
      (return (0.0 0.0 300.0)))))

(fn `GetNavMeshLocation`
  (params (Pawn :type "Pawn Object Reference"))
  (returns (ReturnValue :type "Vector Structure"))
  (locals (DistanceArr :type "Array of Float (double-precision)") (NewLocalVar_0 :type "Array of Float (double-precision)"))
  (bind _distancearr (`local.DistanceArr`))
  (bind _outactors (`GameplayStatics.GetAllActorsOfClass` "/Script/NavigationSystem.NavMeshBoundsVolume"))
  (for _array_element _outactors
    (`KismetArrayLibrary.Array_Add` (`local.DistanceArr`) (`KismetMathLibrary.Vector_Distance` (`Actor.K2_GetActorLocation` _array_element) (`Actor.K2_GetActorLocation` (`local.Pawn`)))))
  (if (> (`KismetArrayLibrary.Array_Length` _distancearr) 0)
    (return (`Actor.K2_GetActorLocation` (`|GetArrayItem` _outactors (`KismetMathLibrary.MinOfFloatArray` _distancearr))))
    (else
      (return (0.0 0.0 0.0)))))

(fn `GetRandomLocation`
  (params (Pawn :type "Pawn Object Reference"))
  (returns (RandomLocation :type "Vector Structure") (ReturnValue :type Boolean))
  (bind (_randomlocation _returnvalue) (`NavigationSystemV1.K2_GetRandomReachablePointInRadius` (`Actor.K2_GetActorLocation` Pawn) (`self.Radius`) null null))
  (`self.SetDefaultNavMeshLocation` Pawn)
  (if (`NavMovementComponent.IsFlying` (`Actor.GetComponentByClass` Pawn "/Script/Engine.CharacterMovementComponent"))
    (return (`KismetMathLibrary.MakeVector` (.x (`KismetMathLibrary.SelectVector` _randomlocation (`self.NavMeshLocation`) _returnvalue)) (.y (`KismetMathLibrary.SelectVector` _randomlocation (`self.NavMeshLocation`) _returnvalue)) (`KismetMathLibrary.RandomFloatInRange` 300.0 1500.0)) true)
    (else
      (return _randomlocation _returnvalue))))

(fn `SetDefaultNavMeshLocation`
  (params (Pawn :type "Pawn Object Reference"))
  (locals (DistanceArr :type "Array of Float (double-precision)") (NewLocalVar_0 :type "Array of Float (double-precision)"))
  (bind _distancearr (`local.DistanceArr`))
  (if (== (`self.NavMeshLocation`) (0.0 0.0 0.0))
    (bind _outactors (`GameplayStatics.GetAllActorsOfClass` "/Script/NavigationSystem.NavMeshBoundsVolume"))
    (for _array_element _outactors
      (`KismetArrayLibrary.Array_Add` (`local.DistanceArr`) (`KismetMathLibrary.Vector_Distance` (`Actor.K2_GetActorLocation` _array_element) (`Actor.K2_GetActorLocation` (`local.Pawn`)))))
    (if (> (`KismetArrayLibrary.Array_Length` _distancearr) 0)
      (set `self.NavMeshLocation` (`Actor.K2_GetActorLocation` (`|GetArrayItem` _outactors (`KismetMathLibrary.MinOfFloatArray` _distancearr)))))))