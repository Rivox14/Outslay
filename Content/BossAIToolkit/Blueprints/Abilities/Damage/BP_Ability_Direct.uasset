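; BP_Ability_Direct is a Boss AI Toolkit damage ability that hits its target actor directly, with no trace or overlap check in this Blueprint.
; On BeginPlay it forces the AI to rotate toward the target's current location.
; When damage begins, it applies ability damage to the target using a constructed non-blocking hit result.
; When damage ends, it disables damage, clears the damaged actors and resets rotation.
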(event `self.ReceiveBeginPlay`
  (`parent.ReceiveBeginPlay`)
  (`self.ForceRotateAI` (`self.K2_GetActorLocation` (`self.TargetActor`))))

(event `self.OnBeginDamage`
  (params (Duration :type "Float (double-precision)"))
  (bind _targetactor (`self.TargetActor`))
  (set `self.CanDealDamage` true)
  (`self.ApplyAbilityDamage` _targetactor (`self.K2_GetActorLocation`) false 0.0 true (`GameplayStatics.MakeHitResult` false false 0.0 0.0 (0.0 0.0 0.0) (0.0 0.0 0.0) (0.0 0.0 1.0) (0.0 0.0 1.0) null _targetactor)))

(event `self.OnEndDamage`
  (set `self.CanDealDamage` false)
  (`KismetArrayLibrary.Array_Clear` (`self.DamagedActors`))
  (`self.ResetRotation`))

(fn `UserConstructionScript`
  (`parent.UserConstructionScript`))