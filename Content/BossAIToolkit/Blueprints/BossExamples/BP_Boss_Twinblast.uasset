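; BP_Boss_Twinblast is an example Twinblast boss from the Boss AI Toolkit that reveals a special gun while using its Ultimate ability.
; The construction script makes the UltGun mesh follow the main Mesh through leader pose and hides it.
; BossBehavior's ability start and end events check for the "Ultimate" name and toggle the gun's visibility through a shared custom event.
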(event `self.Boss Behavior.OnUseAbility`
  (params (AbilityInfo :type "/Game/BossAIToolkit/Blueprints/Structs/F_BossAbility Structure"))
  ;[1 1 1] Show and hide the Ultimate Gun when using the Ultimate ability
  (if (== (`.AbilityName_2_7BDF787B47DAA120ADD0FC99DDFBCE98` (break `/Game/BossAIToolkit/Blueprints/Structs/F_BossAbility` AbilityInfo)) "Ultimate")
    (`self.OnSetUltGunVisibility` true)))

(event `self.Boss Behavior.OnEndAbility`
  (params (AbilityInfo :type "/Game/BossAIToolkit/Blueprints/Structs/F_BossAbility Structure"))
  ;[1 1 1] Show and hide the Ultimate Gun when using the Ultimate ability
  (if (== (`.AbilityName_2_7BDF787B47DAA120ADD0FC99DDFBCE98` (break `/Game/BossAIToolkit/Blueprints/Structs/F_BossAbility` AbilityInfo)) "Ultimate")
    (`self.OnSetUltGunVisibility` false)))

(event `OnSetUltGunVisibility`
  (params (IsVisible :type Boolean))
  ;[1 1 1] Show and hide the Ultimate Gun when using the Ultimate ability
  (`SceneComponent.SetVisibility` (`self.UltGun`) IsVisible false))

(fn `UserConstructionScript`
  (bind _ultgun (`self.UltGun`))
  (`parent.UserConstructionScript`)
  (`SkinnedMeshComponent.SetLeaderPoseComponent` _ultgun (`self.Mesh`) false false)
  (`SceneComponent.SetVisibility` _ultgun false false))