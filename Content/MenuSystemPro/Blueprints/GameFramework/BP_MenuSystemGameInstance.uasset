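; Game instance for Menu System Pro that hosts the settings and save game managers and tracks playtime across levels.
; Init builds both managers from config classes and starts a looping timer that counts only while unpaused.
; Events handle settings JSON files, level opening, batched sound class volumes and two-step delayed settings application.
; When paused, volume and apply requests are forwarded to the Menu System Pro actor instead of using delays.
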(event `self.ReceiveInit`
  (bind _menusystemconfig (`self.MenuSystemConfig`))
  (bind _menusystemconfig_2 (`self.MenuSystemConfig`))
  (bind _settingsmanagerclass (`/Game/MenuSystemPro/Blueprints/Core/PDA_MenuSystemConfig.SettingsManagerClass` _menusystemconfig))
  (bind _savegamemanagerclass (`/Game/MenuSystemPro/Blueprints/Core/PDA_MenuSystemConfig.SaveGameManagerClass` _menusystemconfig_2))
  ;[0.8228 0.1812 0] Init
  (bind _returnvalue (`KismetSystemLibrary.K2_SetTimerDelegate` (delegate `OnIncreasePlayTimer`) 0.01 true))
  (set `self.PlayTimeTimerHandle` _returnvalue)
  (set `self.MenuSystemConfig` (`/Game/MenuSystemPro/Blueprints/Library/BP_MenuSystemLib.GetMenuSystemConfigFromLibrary`))
  (`KismetSystemLibrary.LoadClassAsset_Blocking` _settingsmanagerclass)
  (bind _returnvalue_2 (`|GenericCreateObject` self (`|ConvertAsset` _settingsmanagerclass) _menusystemconfig))
  (bind _output_get (set `self.SettingsManager` (`|ConvertAsset` _returnvalue_2)))
  (`/Game/MenuSystemPro/Blueprints/Settings/BP_SettingsManager.Initialize` (`|ConvertAsset` _output_get))
  (`KismetSystemLibrary.LoadClassAsset_Blocking` _savegamemanagerclass)
  (bind _returnvalue_3 (`|GenericCreateObject` self (`|ConvertAsset` _savegamemanagerclass) _menusystemconfig_2))
  (bind _output_get_2 (set `self.SaveGameManager` (`|ConvertAsset` _returnvalue_3)))
  (`/Game/MenuSystemPro/Blueprints/SaveGame/BP_SaveGameManager.Initialize` (`|ConvertAsset` _output_get_2)))

(event `OnIncreasePlayTimer`
  ;[0.8228 0.1812 0] Playtime Counter
  (if (not (`GameplayStatics.IsGamePaused`))
    (set `self.CurrentPlayTimeTimer` (+ (`self.CurrentPlayTimeTimer`) 0.01))))

(event `/Game/MenuSystemPro/Blueprints/GameFramework/BPI_GameInstanceExtension.OnSetCurrentPlayTime`
  (params (PlayTimeInSeconds :type "Float (double-precision)"))
  ;[0.8228 0.1812 0] Playtime Counter
  (set `self.CurrentPlayTimeTimer` PlayTimeInSeconds))

(event `/Game/MenuSystemPro/Blueprints/GameFramework/BPI_GameInstanceExtension.OnLoadSettingsFromFile`
  (params (Filepath :type "FilePath Structure"))
  ;[0.8228 0.1812 0] Menu System Pro - Settings Manager Save & Load Events. This is implemented here to prevent compiler warnings
  (bind (_outjsonobject _returnvalue) (`JsonBlueprintFunctionLibrary.FromFile` Filepath))
  (if _returnvalue
    (set `/Game/MenuSystemPro/Blueprints/Settings/BP_SettingsManager.CustomSettingsJson` _outjsonobject (`|ConvertAsset` (`self.SettingsManager`)))))

(event `/Game/MenuSystemPro/Blueprints/GameFramework/BPI_GameInstanceExtension.OnSaveSettingsToFile`
  (params (JsonObject :type "JsonObjectWrapper Structure") (Filepath :type "FilePath Structure"))
  ;[0.8228 0.1812 0] Menu System Pro - Settings Manager Save & Load Events. This is implemented here to prevent compiler warnings
  (`JsonBlueprintFunctionLibrary.ToFile` JsonObject Filepath))

(event `/Game/MenuSystemPro/Blueprints/GameFramework/BPI_GameInstanceExtension.OnSetSoundClassVolume`
  (params (SoundClass :type "SoundClass Object Reference") (Volume :type "Float (double-precision)"))
  (bind _soundclasses (`self.SoundClasses`))
  ;[0.8228 0.1812 0] Menu System Pro - Settings Manager Save & Load Events. This is implemented here to prevent compiler warnings
  (if (`GameplayStatics.IsGamePaused`)
    (`/Game/MenuSystemPro/Blueprints/Core/BP_MenuSystemActor.OnSetSoundClassVolume` (`/Game/MenuSystemPro/Blueprints/Library/BP_MenuSystemLib.GetMenuSystemProActorFromLibrary`) SoundClass Volume)
    (else
      (`|ExecutionSequence`
        (:`then_0`
          (`BlueprintMapLibrary.Map_Add` (`self.SoundClasses`) SoundClass Volume))
        (:`then_1`
          (`KismetSystemLibrary.Delay` 0.1)
          (bind _values (`BlueprintMapLibrary.Map_Values` _soundclasses))
          (bind _keys (`BlueprintMapLibrary.Map_Keys` _soundclasses))
          (for (_array_element _array_index) _keys
            (`/Game/MenuSystemPro/Blueprints/Library/BP_MenuSystemLib.SetSoundClassVolumeProperty` _array_element (`|GetArrayItem` _values _array_index))))))))

(event `/Game/MenuSystemPro/Blueprints/GameFramework/BPI_GameInstanceExtension.OnOpenLevel`
  (params (LevelName :type Name) (bAbsolute :type Boolean) (Options :type String))
  ;[0.8228 0.1812 0] Menu System Pro - Save Game Manager
  (`GameplayStatics.OpenLevel` LevelName bAbsolute Options))

(event `/Game/MenuSystemPro/Blueprints/GameFramework/BPI_GameInstanceExtension.OnApplyCustomSettings`
  ;[0.8228 0.1812 0] Menu System Pro - Apply Settings in two delayed steps
  (if (`GameplayStatics.IsGamePaused`)
    (`/Game/MenuSystemPro/Blueprints/Core/BP_MenuSystemActor.OnApplyCustomSettings` (`/Game/MenuSystemPro/Blueprints/Library/BP_MenuSystemLib.GetMenuSystemProActorFromLibrary`) (`|ConvertAsset` (`self.SettingsManager`)))
    (else
      (`/Game/MenuSystemPro/Blueprints/Settings/BP_SettingsManager.PreApplyCustomSettings` (`|ConvertAsset` (`self.SettingsManager`)))
      (`KismetSystemLibrary.Delay` 0.2)
      (`/Game/MenuSystemPro/Blueprints/Settings/BP_SettingsManager.ApplyCustomSettings` (`|ConvertAsset` (`self.SettingsManager`))))))

(fn `GetCurrentLevel`
  (returns (CurrentLevelName :type Name))
  (bind _returnvalue (`GameplayStatics.GetCurrentLevelName` true))
  (return (`KismetStringLibrary.Conv_StringToName` _returnvalue)))

(fn `GetCurrentPlayTime`
  (returns (PlayTimeInSeconds :type "Float (double-precision)"))
  (return (`self.CurrentPlayTimeTimer`)))

(fn `GetSaveGameManager`
  (returns (SaveGameManager :type "/Game/MenuSystemPro/Blueprints/SaveGame/BP_SaveGameManager Soft Object Reference"))
  (return (`self.SaveGameManager`)))

(fn `GetSettingsManager`
  (returns (SettingsManager :type "/Game/MenuSystemPro/Blueprints/Settings/BP_SettingsManager Soft Object Reference"))
  (return (`self.SettingsManager`)))