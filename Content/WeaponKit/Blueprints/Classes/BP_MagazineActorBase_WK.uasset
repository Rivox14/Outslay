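; Base magazine actor for the weapon kit, representing a spawned magazine mesh in the world.
; On BeginPlay it enables or disables physics on the magazine mesh per a spawn flag and, if a lifetime is set, starts a timer that destroys the actor.
; The construction script shows or hides the bullet mesh and its children depending on whether the magazine is full.
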(event `self.ReceiveBeginPlay`
  (`|ExecutionSequence`
    (:`then_0`
      (`PrimitiveComponent.SetSimulatePhysics` (`self.MagazineMesh`) (`self.bSpawnWithPhysics`)))
    (:`then_1`
      (if (> (`self.Lifetime`) 0.01)
        (bind _returnvalue (`KismetSystemLibrary.K2_SetTimerDelegate` (delegate `OnLifetimeEnd`) (`self.Lifetime`) false 0.1))
        (set `self.LifetimeTimerHandle` _returnvalue)))))

(event `OnLifetimeEnd`
  (`self.K2_DestroyActor`))

(fn `UserConstructionScript`
  (`SceneComponent.SetVisibility` (`self.BulletMesh`) (`self.bIsFull`) true))