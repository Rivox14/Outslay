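; House door actor that starts closed when locked and is unlocked through a Tap interaction, opening toolbox key selection if a key is required.
; Unlocking runs a timeline that swings the mesh 90 degrees, in a direction set by the last Indoor or Outdoor trigger the player entered.
; On main doors those triggers also switch the player's camera mode.
; A looping timer refreshes the interaction icon, hiding it once unlocked.
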(event `self.ReceiveBeginPlay`
  (`self.Open_Close Door`)
  (`KismetSystemLibrary.K2_SetTimerDelegate` (delegate `Update Icon`) 0.2 true)
  (`KismetSystemLibrary.Delay` 2.0)
  (add `/Game/Outslay/PlayerCharacter/PlayerCharacter.On IA_Interact` (`/Game/Outslay/Blueprints/Librarys/OS_FunctionLibrary.Get OS Player Character`) (delegate `On IA_Interact_Event`)))

(event `On IA_Interact_Event`
  (params (`Is Pressed` :type Boolean))
  (bind _asplayer_character (`/Game/Outslay/Blueprints/Librarys/OS_FunctionLibrary.Get OS Player Character`))
  (bind _required_key (`self.Required Key`))
  (bind _tap (`self.Tap`))
  (`/Engine/EditorBlueprintResources/StandardMacros.IsValid` _tap
    (:`Is Valid`
      (if (`/Game/InteractionEssentials/Blueprints/Components/InteractionComponent.Can Reach` _tap)
        (if (`self.locked`)
          (if (`|EnumEquality` _required_key "NewEnumerator0")
            (`/Game/InteractionEssentials/Blueprints/Components/InteractionComponent.CE_Interact` _tap `Is Pressed`)
            (else
              (`/Engine/EditorBlueprintResources/StandardMacros.DoOnce` false :!label _label
                (:`Completed`
                  (`/Game/Outslay/PlayerCharacter/PlayerCharacter.CE_OpenToolBox` _asplayer_character true _required_key)
                  (add `/Game/Outslay/PlayerCharacter/UI/HUD/WB_Player.On Tool Use` (`/Game/Outslay/PlayerCharacter/PlayerCharacter.Player WB` _asplayer_character) (delegate `On Tool Use_Event`)))))))))))

(event `Open_Close Door`
  (bind (_relativerotation_roll _relativerotation_pitch _relativerotation_yaw) (`KismetMathLibrary.BreakRotator` (`SceneComponent.RelativeRotation` (`self.StaticMesh`))))
  (set `self.Target Rotation` (`KismetMathLibrary.SelectFloat` 90.0 -90.0 (`self.Player Indoor`)))
  (bind (_direction _alpha) (`Timeline|Door` :!via `PlayFromStart`)
    (:`Update`
      (`SceneComponent.K2_SetRelativeRotation` (`self.StaticMesh`) (`KismetMathLibrary.MakeRotator` 0.0 0.0 (select `bool` (`self.locked`) :`false` (`KismetMathLibrary.Lerp` _relativerotation_yaw (`self.Target Rotation`) _alpha) :`true` (`KismetMathLibrary.Lerp` _relativerotation_yaw 0.0 _alpha) :!type "Float (single-precision)")) false false))))

(event `Update Icon`
  (if (`self.locked`)
    (bind _tap (`self.Tap`)
      (:`then`
        (set `/Game/InteractionEssentials/Blueprints/Components/InteractionComponent.InteractionIconInfo` (make `/Game/InteractionEssentials/Blueprints/Structs/S_ImageInfo` (`/Game/Outslay/Blueprints/Librarys/OS_FunctionLibrary.Get Input Icon` "NewEnumerator7") (0.55 0.55)) _tap)
        (`/Game/InteractionEssentials/Blueprints/Components/InteractionComponent.CE_Set Icon` _tap))
      (:`else`))
    (else
      (bind _tap_2 (`self.Tap`)
        (:`then`
          (`/Game/InteractionEssentials/Blueprints/Components/InteractionComponent.UpdateMarkerVisibility` _tap_2 false))
        (:`else`)))))

(event `self.Tap.OnInteractionStarted`
  (set `self.locked` false)
  (`KismetSystemLibrary.DelayUntilNextTick`)
  (`self.Open_Close Door`)
  (goto _label :!via `Reset`))

(event `On Tool Use_Event`
  (`KismetSystemLibrary.Delay` 0.2)
  (`/Game/InteractionEssentials/Blueprints/Components/InteractionComponent.CE_Interact` (`self.Tap`) true)
  (remove `/Game/Outslay/PlayerCharacter/UI/HUD/WB_Player.On Tool Use` (`/Game/Outslay/PlayerCharacter/PlayerCharacter.Player WB` (`/Game/Outslay/Blueprints/Librarys/OS_FunctionLibrary.Get OS Player Character`)) (delegate `On Tool Use_Event`))
  (`/Game/Outslay/PlayerCharacter/PlayerCharacter.CE_OpenToolBox` (`/Game/Outslay/Blueprints/Librarys/OS_FunctionLibrary.Get OS Player Character`) false "NewEnumerator0"))

(event `Config`
  (`KismetSystemLibrary.Delay` 2.0)
  (`self.K2_AddActorWorldOffset` (0.0 0.0 1.0))
  (`KismetSystemLibrary.Delay` 2.0)
  (`self.K2_AddActorWorldOffset` (0.0 0.0 -1.0)))

(event `self.Indoor.OnComponentBeginOverlap`
  (params (OverlappedComponent :type "PrimitiveComponent Object Reference") (OtherActor :type "Actor Object Reference") (OtherComp :type "PrimitiveComponent Object Reference") (OtherBodyIndex :type Integer) (bFromSweep :type Boolean) (SweepResult :type "HitResult Structure (by ref)"))
  (bind _asplayer_character (cast `/Game/Outslay/PlayerCharacter/PlayerCharacter` OtherActor))
  (set `self.Player Indoor` true)
  (if (`self.Is MainDoor`)
    (`/Game/Outslay/PlayerCharacter/PlayerCharacter.Set Camera Mode` _asplayer_character true)))

(event `self.Outdoor.OnComponentBeginOverlap`
  (params (OverlappedComponent :type "PrimitiveComponent Object Reference") (OtherActor :type "Actor Object Reference") (OtherComp :type "PrimitiveComponent Object Reference") (OtherBodyIndex :type Integer) (bFromSweep :type Boolean) (SweepResult :type "HitResult Structure (by ref)"))
  (bind _asplayer_character (cast `/Game/Outslay/PlayerCharacter/PlayerCharacter` OtherActor))
  (set `self.Player Indoor` false)
  (if (`self.Is MainDoor`)
    (`/Game/Outslay/PlayerCharacter/PlayerCharacter.Set Camera Mode` _asplayer_character false)))

(fn `UserConstructionScript`)