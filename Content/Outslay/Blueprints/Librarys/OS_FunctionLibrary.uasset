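; Blueprint function library for Outslay with shared helpers for input prompts, player access and skill levels.
; GetInputIcon maps each input action to a button texture for the device read from OS_PlayerController, which defaults to Keyboard if the cast fails.
; Getters return the first OS_PlayerState and PlayerCharacter via casts.
; GetCurrentSkillLevel looks up a skill's value by name in the player state's Skills map.
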(fn `Get Current Skill Level`
  (params (Skill :type "/Game/Outslay/Blueprints/Data/Enum/OS_Skills Enum" :default "NewEnumerator0"))
  (returns (Level :type Integer))
  (bind _skills (`/Game/Outslay/Blueprints/Core/OS_PlayerState.Skills` (`self.Get OS Player State` null)))
  (switch `/Game/Outslay/Blueprints/Data/Enum/OS_Skills` Skill
    (:`NewEnumerator0`
      (return (`BlueprintMapLibrary.Map_Find` _skills "Health Skill")))
    (:`NewEnumerator1`
      (return (`BlueprintMapLibrary.Map_Find` _skills "Stamina Skill")))
    (:`NewEnumerator2`
      (return (`BlueprintMapLibrary.Map_Find` _skills "Inventory Skill")))
    (:`NewEnumerator3`
      (return (`BlueprintMapLibrary.Map_Find` _skills "Ammo Skill")))
    (:`NewEnumerator4`
      (return (`BlueprintMapLibrary.Map_Find` _skills "Damage Skill")))))

(fn `Get Input Device`
  (returns (`Input Device` :type "/Game/Outslay/Input/E_InputDevice_Type Enum"))
  (bind _asos_player_controller (cast `/Game/Outslay/Blueprints/Core/OS_PlayerController` (`GameplayStatics.GetPlayerController` null))
    (:`then`
      (return (`/Game/Outslay/Blueprints/Core/OS_PlayerController.Input Device` _asos_player_controller)))
    (:`CastFailed`
      (return "NewEnumerator0"))))

(fn `Get Input Icon`
  (params (Input :type "/Game/Outslay/Input/E_Input Enum" :default "NewEnumerator0"))
  (returns (NewParam :type "Texture2D Object Reference"))
  (switch `/Game/Outslay/Input/E_InputDevice_Type` (`self.Get Input Device` null)
    (:`NewEnumerator0`
      (switch `/Game/Outslay/Input/E_Input` (`local.Input`)
        (:`NewEnumerator0`
          (return null))
        (:`NewEnumerator1`
          (return null))
        (:`NewEnumerator2`
          (return "/Game/InteractionEssentials/Textures/Input/Micro_Icons/PC_Controller/Dark/T_PC_Space_Dark_64x64.T_PC_Space_Dark_64x64"))
        (:`NewEnumerator3`
          (return "/Game/InteractionEssentials/Textures/Input/Micro_Icons/PC_Controller/Dark/T_PC_Shift_Dark_64x64.T_PC_Shift_Dark_64x64"))
        (:`NewEnumerator4`
          (return "/Game/InteractionEssentials/Textures/Input/Micro_Icons/PC_Controller/Dark/T_PC_Ctrl_Dark_64x64.T_PC_Ctrl_Dark_64x64"))
        (:`NewEnumerator9`
          (return "/Game/InteractionEssentials/Textures/Input/Micro_Icons/PC_Controller/Dark/T_PC_RMB_Dark_64x64.T_PC_RMB_Dark_64x64"))
        (:`NewEnumerator5`
          (return "/Game/InteractionEssentials/Textures/Input/Micro_Icons/PC_Controller/Dark/T_PC_LMB_Dark_64x64.T_PC_LMB_Dark_64x64"))
        (:`NewEnumerator6`
          (return "/Game/InteractionEssentials/Textures/Input/Micro_Icons/PC_Controller/Dark/T_PC_R_Dark_64x64.T_PC_R_Dark_64x64"))
        (:`NewEnumerator7`
          (return "/Game/InteractionEssentials/Textures/Input/Micro_Icons/PC_Controller/Dark/T_PC_F_Dark_64x64.T_PC_F_Dark_64x64"))
        (:`NewEnumerator10`
          (return "/Game/InteractionEssentials/Textures/Input/Micro_Icons/PC_Controller/Dark/T_PC_Tab_Dark_64x64.T_PC_Tab_Dark_64x64"))
        (:`NewEnumerator11`
          (return "/Game/InteractionEssentials/Textures/Input/Micro_Icons/PC_Controller/Light/T_PC_E_Light_64x64.T_PC_E_Light_64x64"))
        (:`NewEnumerator12`
          (return "/Game/InteractionEssentials/Textures/Input/Micro_Icons/PC_Controller/Light/T_PC_Q_Light_64x64.T_PC_Q_Light_64x64"))
        (:`NewEnumerator15`
          (return "/Game/InteractionEssentials/Textures/Input/Micro_Icons/PC_Controller/Light/T_PC_I_Light_64x64.T_PC_I_Light_64x64"))
        (:`NewEnumerator16`
          (return "/Game/InteractionEssentials/Textures/Input/Micro_Icons/PC_Controller/Light/T_PC_Space2_Light_64x64.T_PC_Space2_Light_64x64"))
        (:`NewEnumerator17`
          (return "/Game/InteractionEssentials/Textures/Input/Micro_Icons/PC_Controller/Light/T_PC_Esc_Light_64x64.T_PC_Esc_Light_64x64"))))
    (:`NewEnumerator1`
      (switch `/Game/Outslay/Input/E_Input` (`local.Input`)
        (:`NewEnumerator0`
          (return "/Game/InteractionEssentials/Textures/Input/Micro_Icons/XB_Controller/Dark/T_XB_LS_Dark_64x64.T_XB_LS_Dark_64x64"))
        (:`NewEnumerator1`
          (return "/Game/InteractionEssentials/Textures/Input/Micro_Icons/XB_Controller/Dark/T_XB_RS_Dark_64x64.T_XB_RS_Dark_64x64"))
        (:`NewEnumerator2`
          (return "/Game/InteractionEssentials/Textures/Input/Micro_Icons/XB_Controller/Dark/T_XB_A_Dark_64x64.T_XB_A_Dark_64x64"))
        (:`NewEnumerator3`
          (return "/Game/InteractionEssentials/Textures/Input/Micro_Icons/XB_Controller/Dark/T_XB_Base_LB_Dark_64x64.T_XB_Base_LB_Dark_64x64"))
        (:`NewEnumerator4`
          (return "/Game/InteractionEssentials/Textures/Input/Micro_Icons/XB_Controller/Dark/T_XB_LS_L3_Dark_64x64.T_XB_LS_L3_Dark_64x64"))
        (:`NewEnumerator9`
          (return "/Game/InteractionEssentials/Textures/Input/Micro_Icons/XB_Controller/Dark/T_XB_Base_LT_Dark_64x64.T_XB_Base_LT_Dark_64x64"))
        (:`NewEnumerator5`
          (return "/Game/InteractionEssentials/Textures/Input/Micro_Icons/XB_Controller/Dark/T_XB_Base_RT_Dark_64x64.T_XB_Base_RT_Dark_64x64"))
        (:`NewEnumerator6`
          (return "/Game/InteractionEssentials/Textures/Input/Micro_Icons/XB_Controller/Dark/T_XB_B_Dark_64x64.T_XB_B_Dark_64x64"))
        (:`NewEnumerator7`
          (return "/Game/InteractionEssentials/Textures/Input/Micro_Icons/XB_Controller/Dark/T_XB_Y_Dark_64x64.T_XB_Y_Dark_64x64"))
        (:`NewEnumerator10`
          (return "/Game/InteractionEssentials/Textures/Input/Micro_Icons/XB_Controller/Dark/T_XB_Base_RB_Dark_64x64.T_XB_Base_RB_Dark_64x64"))
        (:`NewEnumerator11`
          (return "/Game/InteractionEssentials/Textures/Input/Micro_Icons/XB_Controller/Light/T_XB_Base_RT_Light_64x64.T_XB_Base_RT_Light_64x64"))
        (:`NewEnumerator12`
          (return "/Game/InteractionEssentials/Textures/Input/Micro_Icons/XB_Controller/Light/T_XB_Base_LT_Light_64x64.T_XB_Base_LT_Light_64x64"))
        (:`NewEnumerator15`
          (return "/Game/InteractionEssentials/Textures/Input/Micro_Icons/XB_Controller/Light/T_XB_Dpad_R_Light_64x64.T_XB_Dpad_R_Light_64x64"))
        (:`NewEnumerator16`
          (return "/Game/InteractionEssentials/Textures/Input/Micro_Icons/XB_Controller/Dark/T_XB_A_Dark_64x64.T_XB_A_Dark_64x64"))
        (:`NewEnumerator17`
          (return "/Game/InteractionEssentials/Textures/Input/Micro_Icons/XB_Controller/Dark/T_XB_B_Dark_64x64.T_XB_B_Dark_64x64"))))
    (:`NewEnumerator2`
      (switch `/Game/Outslay/Input/E_Input` (`local.Input`)
        (:`NewEnumerator0`
          (return null))
        (:`NewEnumerator1`
          (return null))
        (:`NewEnumerator2`
          (return "/Game/Survival-UI-Bundle/PC_and_Console_Controls/Console_P_Constrols/CROSS.CROSS"))
        (:`NewEnumerator3`
          (return "/Game/Survival-UI-Bundle/PC_and_Console_Controls/Console_P_Constrols/L1.L1"))
        (:`NewEnumerator4`
          (return "/Game/InteractionEssentials/Textures/Input/Micro_Icons/XB_Controller/Dark/T_XB_LS_L3_Dark_64x64.T_XB_LS_L3_Dark_64x64"))
        (:`NewEnumerator9`
          (return "/Game/Survival-UI-Bundle/PC_and_Console_Controls/Console_P_Constrols/L2.L2"))
        (:`NewEnumerator5`
          (return "/Game/Survival-UI-Bundle/PC_and_Console_Controls/Console_P_Constrols/R2.R2"))
        (:`NewEnumerator6`
          (return "/Game/Survival-UI-Bundle/PC_and_Console_Controls/Console_P_Constrols/CIRCLE.CIRCLE"))
        (:`NewEnumerator7`
          (return "/Game/Survival-UI-Bundle/PC_and_Console_Controls/Console_P_Constrols/TRIANGLE.TRIANGLE"))
        (:`NewEnumerator10`
          (return "/Game/Survival-UI-Bundle/PC_and_Console_Controls/Console_P_Constrols/R1.R1"))
        (:`NewEnumerator11`
          (return "/Game/Survival-UI-Bundle/PC_and_Console_Controls/Console_P_Constrols/R2.R2"))
        (:`NewEnumerator12`
          (return "/Game/Survival-UI-Bundle/PC_and_Console_Controls/Console_P_Constrols/L2.L2"))
        (:`NewEnumerator15`
          (return "/Game/InteractionEssentials/Textures/Input/Micro_Icons/XB_Controller/Light/T_XB_Dpad_R_Light_64x64.T_XB_Dpad_R_Light_64x64"))
        (:`NewEnumerator16`
          (return "/Game/InteractionEssentials/Textures/Input/Micro_Icons/XB_Controller/Dark/T_XB_X_Dark_64x64.T_XB_X_Dark_64x64"))
        (:`NewEnumerator17`
          (return "/Game/Survival-UI-Bundle/PC_and_Console_Controls/Console_P_Constrols/CIRCLE.CIRCLE"))))))

(fn `Get OS Player Character`
  (returns (`AsPlayer Character` :type "/Game/Outslay/PlayerCharacter/PlayerCharacter Object Reference"))
  (bind _asplayer_character (cast `/Game/Outslay/PlayerCharacter/PlayerCharacter` (`GameplayStatics.GetPlayerCharacter` null)))
  (return _asplayer_character))

(fn `Get OS Player State`
  (returns (`AsOS Player State` :type "/Game/Outslay/Blueprints/Core/OS_PlayerState Object Reference"))
  (bind _asos_player_state (cast `/Game/Outslay/Blueprints/Core/OS_PlayerState` (`GameplayStatics.GetPlayerState` null)))
  (return _asos_player_state))