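; BP_Bow is the player's bow weapon, firing BP_Arrow rounds through the EBBarrel component.
; While held, it follows aim and movement events to connect or disconnect the bow component, forcing walking when aiming and disconnecting on crouch.
; A cosmetic arrow attaches to the mesh when loaded and is destroyed on firing.
; DoOnce and delays pace shots, and each shot auto-reloads from reserve ammo and updates inventory.
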(event `self.ReceiveBeginPlay`
  (bind _asplayer_character (`/Game/Outslay/Blueprints/Librarys/OS_FunctionLibrary.Get OS Player Character`))
  (`parent.ReceiveBeginPlay`)
  (`KismetArrayLibrary.Array_Add` (`EBBarrel.Ammo` (`self.EBBarrel`)) "/Game/Outslay/Blueprints/Items/Weapons/Bow/BP_Arrow.BP_Arrow_C")
  (`/Engine/EditorBlueprintResources/StandardMacros.IsValid` _asplayer_character
    (:`Is Valid`
      (add `/Game/Outslay/PlayerCharacter/PlayerCharacter.On Held Item Change` _asplayer_character (delegate `On Held Item Change_Event`)))))

(event `On Held Item Change_Event`
  (params (`Held Item` :type "/Game/Outslay/Blueprints/Items/OS_ItemBase Object Reference"))
  (bind _asplayer_character (`/Game/Outslay/Blueprints/Librarys/OS_FunctionLibrary.Get OS Player Character`))
  (bind _ct_cmpt_locomotion (`/Game/Outslay/PlayerCharacter/PlayerCharacter.CT_Cmpt_Locomotion` _asplayer_character))
  (if (== `Held Item` self)
    (add `/Game/Outslay/PlayerCharacter/PlayerCharacter.On Aim` _asplayer_character (delegate `On Aim_Event`))
    (add `/Game/LocomotionSystem/Assets/CT_Components/LocomotionSystem/Components/CT_Cmpt_Locomotion.Event_OnSetMovementType` _ct_cmpt_locomotion (delegate `Event_OnSetMovementType_Event`))
    (else
      (remove `/Game/Outslay/PlayerCharacter/PlayerCharacter.On Aim` _asplayer_character (delegate `On Aim_Event`))
      (remove `/Game/LocomotionSystem/Assets/CT_Components/LocomotionSystem/Components/CT_Cmpt_Locomotion.Event_OnSetMovementType` _ct_cmpt_locomotion (delegate `Event_OnSetMovementType_Event`)))))

(event `Event_OnSetMovementType_Event`
  (params (MovementType :type "/Game/LocomotionSystem/Assets/CT_Components/LocomotionSystem/Datas/Enumerations/Enum_MovementType Enum" :default "NewEnumerator4"))
  (switch `/Game/LocomotionSystem/Assets/CT_Components/LocomotionSystem/Datas/Enumerations/Enum_MovementType` MovementType
    (:`NewEnumerator3`
      (`/Game/LocomotionSystem/Blueprints/Components/CT_Cmpt_Bow_Lite.SetBowStatus` (`self.CT_Cmpt_Bow_Lite`) "NewEnumerator1"))))

(event `On Aim_Event`
  (params (`Held Item` :type Name) (Aim :type Boolean))
  (bind _asplayer_character (`/Game/Outslay/Blueprints/Librarys/OS_FunctionLibrary.Get OS Player Character`))
  (`|ExecutionSequence`
    (:`then_0`
      (set `self.Aiming` Aim)
      (`KismetSystemLibrary.RetriggerableDelay` (`KismetMathLibrary.SelectFloat` 0.0 1.4 Aim))
      (if Aim
        (`|ExecutionSequence`
          (:`then_0`
            (`/Engine/EditorBlueprintResources/StandardMacros.IsValid` _asplayer_character
              (:`Is Valid`
                (`/Game/Outslay/PlayerCharacter/PlayerCharacter.CE_UnCrouch` _asplayer_character))))
          (:`then_1`
            (switch `/Game/LocomotionSystem/Blueprints/Datas/Enumerations/Enum_BowStatus` (`/Game/LocomotionSystem/Blueprints/Components/CT_Cmpt_Bow_Lite.BowStatus` (`self.CT_Cmpt_Bow_Lite`))
              (:`NewEnumerator1`
                _)
              (:`NewEnumerator2`
                _))
            (`GameplayStatics.PlaySoundAtLocation` "/Game/The_Sound_Of_Survival_Vol1/CUE/Weapons/Bow/Bow_Handling/CUE_Bow_Handling_01_Cue.CUE_Bow_Handling_01_Cue" (`self.K2_GetActorLocation`) (struct) 1.0 1.0 0.0 null null null null))
          (:`then_2`
            (`KismetSystemLibrary.RetriggerableDelay` 0.2)
            (`/Game/LocomotionSystem/Blueprints/Components/CT_Cmpt_Bow_Lite.SetBowStatus` (`self.CT_Cmpt_Bow_Lite`) "NewEnumerator0")
            (`KismetSystemLibrary.RetriggerableDelay` 0.3)
            (`self.Make Arrow`)))
        (else
          (`/Game/LocomotionSystem/Blueprints/Components/CT_Cmpt_Bow_Lite.SetBowStatus` (`self.CT_Cmpt_Bow_Lite`) "NewEnumerator1")
          (bind _arrow_actor (`self.Arrow Actor`)
            (:`then`
              (`self.K2_DestroyActor` _arrow_actor))
            (:`else`)))))
    (:`then_1`
      (if Aim
        (`/Game/LocomotionSystem/Assets/CT_Components/LocomotionSystem/Components/CT_Cmpt_Locomotion.SetMovementType` (`/Game/Outslay/PlayerCharacter/PlayerCharacter.CT_Cmpt_Locomotion` (`/Game/Outslay/Blueprints/Librarys/OS_FunctionLibrary.Get OS Player Character`)) "NewEnumerator0")))))

(event `Make Arrow`
  (bind (_returnvalue_location _returnvalue_rotation) (`KismetMathLibrary.BreakTransform` (`SceneComponent.K2_GetComponentToWorld` (`self.Muzzel`))))
  (if (> (`self.Loaded Ammo`) 0)
    (`self.Arrow Actor`
      (:`then`)
      (:`else`
        (bind _returnvalue (`|SpawnActorFromClass` "/Game/Outslay/Blueprints/Items/Weapons/Bow/Arrow_Mesh.Arrow_Mesh_C" (`KismetMathLibrary.MakeTransform` _returnvalue_location _returnvalue_rotation (1.15 1.0 1.0)) "AlwaysSpawn" "OverrideRootScale" self null))
        (set `self.Arrow Actor` _returnvalue)
        (`self.K2_AttachToComponent` (`self.Arrow Actor`) (`self.ItemMesh`) "Arrow" "SnapToTarget" "SnapToTarget" "KeepRelative" true)))))

(event `Bow Fire`
  (bind _returnvalue (`self.K2_GetActorLocation`))
  (`/Engine/EditorBlueprintResources/StandardMacros.DoOnce` false :!label _label
    (:`Completed`
      (`|ExecutionSequence`
        (:`then_0`
          (`/Game/LocomotionSystem/Blueprints/Components/CT_Cmpt_Bow_Lite.SetBowStatus` (`self.CT_Cmpt_Bow_Lite`) "NewEnumerator2")
          (`/Game/Outslay/PlayerCharacter/PlayerCharacter.CE_Play Fire Montage` (`/Game/Outslay/Blueprints/Librarys/OS_FunctionLibrary.Get OS Player Character`))
          (`|ExecutionSequence`
            (:`then_0`
              (`KismetSystemLibrary.Delay` 0.4)
              (`/Game/LocomotionSystem/Blueprints/Components/CT_Cmpt_Bow_Lite.SetBowStatus` (`self.CT_Cmpt_Bow_Lite`) "NewEnumerator0")
              (`GameplayStatics.PlaySoundAtLocation` "/Game/The_Sound_Of_Survival_Vol1/CUE/Weapons/Bow/Bow_Handling/CUE_Bow_Handling_01_Cue.CUE_Bow_Handling_01_Cue" (`self.K2_GetActorLocation`) (struct) 1.0 1.0 0.3 null null null null)
              (`KismetSystemLibrary.Delay` 0.2)
              (if (`self.Aiming`)
                (`self.Make Arrow`)))
            (:`then_1`
              (bind _arrow_actor (`self.Arrow Actor`)
                (:`then`
                  (`GameplayStatics.PlaySoundAtLocation` "/Game/WeaponKit/FX/A_Bow_FireArrow_WK.A_Bow_FireArrow_WK" _returnvalue (struct) 1.0 1.0 0.0 null null null null)
                  (`self.K2_DestroyActor` _arrow_actor)
                  (set `self.Arrow Actor` null)
                  (`EBBarrel.Shoot` (`self.EBBarrel`) true))
                (:`else`
                  (`GameplayStatics.PlaySoundAtLocation` "/Game/WeaponKit/FX/A_Bow_FireDry_WK.A_Bow_FireDry_WK" _returnvalue (struct) 1.0 1.0 0.0 null null null null))))))
        (:`then_1`
          (`KismetSystemLibrary.Delay` 0.94)
          (goto _label :!via `Reset`))))))

(event `self.ReceiveDestroyed`
  (bind _arrow_actor (`self.Arrow Actor`)
    (:`then`
      (`self.K2_DestroyActor` _arrow_actor))
    (:`else`)))

(event `Update Ammo`
  (`/Engine/EditorBlueprintResources/StandardMacros.DecrementInt` (`self.Loaded Ammo`)
    (:`  `
      (`/Engine/EditorBlueprintResources/StandardMacros.DoOnce` false :!label _label_2
        (:`Completed`
          (if (`self.Can Reload`)
            (`|ExecutionSequence`
              (:`then_0`
                (set `self.Reloading` true)
                (if (> (`self.Ammo`) (`self.Mag Size`))
                  (set `self.Ammo` (- (`self.Ammo`) (- (`self.Mag Size`) (`self.Loaded Ammo`))))
                  (set `self.Loaded Ammo` (`self.Mag Size`))
                  (`/Game/Outslay/PlayerCharacter/PlayerCharacter.Update Inventory` (`/Game/Outslay/Blueprints/Librarys/OS_FunctionLibrary.Get OS Player Character`))
                  (else
                    (set `self.Loaded Ammo` (`self.Ammo`))
                    (set `self.Ammo` 0)
                    (`/Game/Outslay/PlayerCharacter/PlayerCharacter.Update Inventory` (`/Game/Outslay/Blueprints/Librarys/OS_FunctionLibrary.Get OS Player Character`)))))
              (:`then_1`
                (`KismetSystemLibrary.RetriggerableDelay` 0.2)
                (set `self.Reloading` false)
                (`KismetSystemLibrary.RetriggerableDelay` 0.2)
                (goto _label_2 :!via `Reset`)))
            (else
              (`/Game/Outslay/PlayerCharacter/PlayerCharacter.Update Inventory` (`/Game/Outslay/Blueprints/Librarys/OS_FunctionLibrary.Get OS Player Character`)))))))))

(event `self.EBBarrel.ShotFired`
  (`self.Update Ammo`)
  (`EBBarrel.Shoot` (`self.EBBarrel`) false))

(fn `UserConstructionScript`
  (`parent.UserConstructionScript`))