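; BP_Ammo is an ammo item actor whose appearance follows its AmmoType: pistol, rifle, shotgun, arrow or launcher.
; The construction script calls the parent, then selects the matching static mesh for ItemMesh and applies a per-type vertical offset.
; It also copies Ammo into CurrentAmount.
; The event graph holds only disabled placeholder events, so the Blueprint adds no runtime logic of its own.
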(fn `UserConstructionScript`
  (`parent.UserConstructionScript`)
  (`StaticMeshComponent.SetStaticMesh` (`self.ItemMesh`) (select `/Game/Outslay/Blueprints/Items/RowItem/Ammo/E_AmmoType` (`self.Ammo Type`) :`NewEnumerator0` "/Game/Ammo_boxes/Props/Open_boxes_with_ammo/SM_45_open_dirty_with_ammo.SM_45_open_dirty_with_ammo" :`NewEnumerator1` "/Game/Ammo_boxes/Props/Open_boxes_with_ammo/SM_7_62x54_open_dirty_with_ammo.SM_7_62x54_open_dirty_with_ammo" :`NewEnumerator2` "/Game/Ammo_boxes/Props/Open_boxes_with_ammo/SM_12x76_open_dirty_with_ammo.SM_12x76_open_dirty_with_ammo" :`NewEnumerator3` "/Game/Ammo_boxes/Props/Piles_of_ammo/SM_Pile_arrows_dirty.SM_Pile_arrows_dirty" :`NewEnumerator4` "/Game/WeaponKit/Bullets/RocketLauncher.RocketLauncher" :!type "StaticMesh Object Reference"))
  (`SceneComponent.K2_SetRelativeLocation` (`self.ItemMesh`) (`KismetMathLibrary.MakeVector` 0.0 0.0 (select `/Game/Outslay/Blueprints/Items/RowItem/Ammo/E_AmmoType` (`self.Ammo Type`) :`NewEnumerator3` 1.0 :`NewEnumerator4` 3.0)) false false)
  (set `self.Current Amount` (`self.Ammo`)))