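; Base actor for Outslay's items, handling pickup through a Tap interaction component that is switched off while the item is held.
; Interaction start turns the player toward the item, switches to fists for weapon pickups and plays a stance- and height-matched harvest montage.
; Completion drops any third-slot melee weapon as a physics actor keeping its durability, adds the item, equips weapons, then destroys itself.
; Timed delays sync both stages with holstering and animation.
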(event `self.Tap.OnInteractionCompleted`
  (bind _asplayer_character (`/Game/Outslay/Blueprints/Librarys/OS_FunctionLibrary.Get OS Player Character`))
  (bind _asplayer_character_2 (`/Game/Outslay/Blueprints/Librarys/OS_FunctionLibrary.Get OS Player Character`))
  (bind ((`MeleeWeapons_45_12A04DD749A3592FA21E1590EB7AD030` _meleeweapons)) (break `/Game/Outslay/PlayerCharacter/UI/Inventory/Data/S_Inventory_Data` (`/Game/Outslay/Blueprints/Core/OS_PlayerState.Inventory` (`/Game/Outslay/Blueprints/Librarys/OS_FunctionLibrary.Get OS Player State`))))
  (bind (_returnvalue_location _returnvalue_rotation) (`KismetMathLibrary.BreakTransform` (`self.GetTransform` (`/Game/Outslay/PlayerCharacter/PlayerCharacter.Get Held Item` _asplayer_character))))
  (bind (_output_name _output_currentamount _output_maxamount _output_itemimage _output_durability) (break `/Game/Outslay/PlayerCharacter/UI/Inventory/Data/S_InventoryItem` (`|GetArrayItem` _meleeweapons 2)))
  (if (`/Game/Outslay/Blueprints/Core/OS_PlayerState.Can Add Item` (`/Game/Outslay/Blueprints/Librarys/OS_FunctionLibrary.Get OS Player State`) self)
    (if (`self.Should  Wait`)
      (`KismetSystemLibrary.Delay` 0.7))
    (`|ExecutionSequence`
      (:`then_0`
        (if (`|EnumEquality` (`self.Item Type`) "NewEnumerator2")
          (if (`KismetArrayLibrary.Array_Contains` (`|MakeArray` "Fist" "Knife") (`self.Item Name`))
            _
            (elif (`KismetArrayLibrary.Array_IsValidIndex` _meleeweapons 2)
              (`|SpawnActorFromClass` (`self.Get Class` _output_name) (`KismetMathLibrary.MakeTransform` (+ (* (`self.GetActorForwardVector` _asplayer_character) 36.0) _returnvalue_location) _returnvalue_rotation) "AdjustIfPossibleButAlwaysSpawn" "MultiplyWithRoot" null _output_durability true "NewEnumerator1" null)))))
      (:`then_1`
        (`/Game/Outslay/Blueprints/Core/OS_PlayerState.Add Item` (`/Game/Outslay/Blueprints/Librarys/OS_FunctionLibrary.Get OS Player State`) self)
        (`|ExecutionSequence`
          (:`then_0`
            (if (or (`|EnumEquality` (`self.Item Type`) "NewEnumerator2") (`|EnumEquality` (`self.Item Type`) "NewEnumerator0") (`|EnumEquality` (`self.Item Type`) "NewEnumerator1"))
              (`/Game/Outslay/PlayerCharacter/PlayerCharacter.Equip Item` _asplayer_character_2 (`self.Item Name`) false true)
              (`/Game/Outslay/PlayerCharacter/PlayerCharacter.Update Item Wheel` _asplayer_character_2 (`self.Item Type`) (`self.Item Name`))))
          (:`then_1`
            (`KismetSystemLibrary.Delay` 0.56)
            (`|ExecutionSequence`
              (:`then_0`
                (`KismetSystemLibrary.Delay` 0.02)
                (`SceneComponent.SetVisibility` (`self.DefaultSceneRoot`) false true)
                (`GameplayStatics.PlaySoundAtLocation` (`self.Pickup Sound`) (`SceneComponent.K2_GetComponentLocation` (`self.DefaultSceneRoot`)) (struct) 1.0 1.0 0.0 null null null null))
              (:`then_1`
                (`KismetSystemLibrary.Delay` (select `/Game/Outslay/PlayerCharacter/UI/ItemWheel/Data/E_ItemType` (`self.Item Type`) :`NewEnumerator3` 0.7 :`NewEnumerator4` 0.7 :`NewEnumerator6` 0.7 :!type "Float (single-precision)"))
                (`SceneComponent.SetVisibility` (`/Game/Outslay/PlayerCharacter/PlayerCharacter.ChildActor` (`/Game/Outslay/Blueprints/Librarys/OS_FunctionLibrary.Get OS Player Character`)) true false)
                (`KismetSystemLibrary.Delay` 0.4)
                (`self.K2_DestroyActor`)))))))))

(event `self.ReceiveBeginPlay`
  (set `/Game/InteractionEssentials/Blueprints/Components/InteractionComponent.InteractionIconInfo` (make `/Game/InteractionEssentials/Blueprints/Structs/S_ImageInfo` (`/Game/Outslay/Blueprints/Librarys/OS_FunctionLibrary.Get Input Icon` "NewEnumerator7") (0.55 0.55)) (`self.Tap`))
  (`KismetSystemLibrary.Delay` 2.0)
  (add `/Game/Outslay/PlayerCharacter/PlayerCharacter.On IA_Interact` (`/Game/Outslay/Blueprints/Librarys/OS_FunctionLibrary.Get OS Player Character`) (delegate `On IA_Interact_Event`)))

(event `On IA_Interact_Event`
  (params (`Is Pressed` :type Boolean))
  (bind _tap (`self.Tap`))
  (`/Engine/EditorBlueprintResources/StandardMacros.IsValid` _tap
    (:`Is Valid`
      (if (`/Game/InteractionEssentials/Blueprints/Components/InteractionComponent.Can Reach` _tap)
        (`/Game/InteractionEssentials/Blueprints/Components/InteractionComponent.CE_Interact` _tap `Is Pressed`)))))

(event `self.Tap.OnInteractionStarted`
  (bind _asplayer_character (`/Game/Outslay/Blueprints/Librarys/OS_FunctionLibrary.Get OS Player Character`))
  (bind _returnvalue (`self.GetComponentByClass` "/Script/Engine.SkeletalMeshComponent"))
  (bind _returnvalue_2 (`self.GetComponentByClass` "/Script/Engine.StaticMeshComponent"))
  (bind _asplayer_character_2 (`/Game/Outslay/Blueprints/Librarys/OS_FunctionLibrary.Get OS Player Character`))
  (bind (_returnvalue_roll _returnvalue_pitch) (`KismetMathLibrary.BreakRotator` (`self.K2_GetActorRotation` _asplayer_character_2)))
  (bind (_item _item_type) (`/Game/Outslay/PlayerCharacter/PlayerCharacter.Get Held Item` (`/Game/Outslay/Blueprints/Librarys/OS_FunctionLibrary.Get OS Player Character`)))
  (bind (_returnvalue_roll_2 _returnvalue_pitch_2 _returnvalue_yaw) (`KismetMathLibrary.BreakRotator` (`KismetMathLibrary.FindLookAtRotation` (`self.K2_GetActorLocation` _asplayer_character_2) (`SceneComponent.K2_GetComponentLocation` (select `bool` (`KismetSystemLibrary.IsValid` _returnvalue) :`false` (select `bool` (`KismetSystemLibrary.IsValid` _returnvalue_2) :`false` (`self.DefaultSceneRoot`) :`true` _returnvalue_2 :!type "SceneComponent Object Reference") :`true` _returnvalue :!type "SceneComponent Object Reference")))))
  (if (`/Game/Outslay/Blueprints/Core/OS_PlayerState.Can Add Item` (`/Game/Outslay/Blueprints/Librarys/OS_FunctionLibrary.Get OS Player State`) self)
    (`|ExecutionSequence`
      (:`then_0`
        (`self.K2_SetActorRotation` _asplayer_character_2 (`KismetMathLibrary.MakeRotator` _returnvalue_roll _returnvalue_pitch _returnvalue_yaw) false)
        (`|ExecutionSequence`
          (:`then_0`
            (if (or (`|EnumEquality` (`self.Item Type`) "NewEnumerator2") (`|EnumEquality` (`self.Item Type`) "NewEnumerator0") (`|EnumEquality` (`self.Item Type`) "NewEnumerator1"))
              (`/Game/Outslay/PlayerCharacter/PlayerCharacter.Equip Item` (`/Game/Outslay/Blueprints/Librarys/OS_FunctionLibrary.Get OS Player Character`) "Fist" (select `bool` (== (`/Game/Outslay/Blueprints/Items/OS_ItemBase.Item Name` _item) "Bow") :`false` (select `/Game/Outslay/PlayerCharacter/UI/ItemWheel/Data/E_ItemType` _item_type :`NewEnumerator0` true :`NewEnumerator1` true)) true)))
          (:`then_1`
            (if (`self.Should  Wait`)
              (`KismetSystemLibrary.Delay` 0.7))
            (switch `/Game/LocomotionSystem/Assets/CT_Components/LocomotionSystem/Datas/Enumerations/Enum_MovementType` (`/Game/LocomotionSystem/Assets/CT_Components/LocomotionSystem/Components/CT_Cmpt_Locomotion.GetMovementType` (`/Game/Outslay/PlayerCharacter/PlayerCharacter.CT_Cmpt_Locomotion` _asplayer_character))
              (:`NewEnumerator4`
                (switch `/Game/Outslay/Blueprints/Items/Data/E_ItempPos` (`self.Item Location`) :!label _label
                  (:`NewEnumerator0`
                    (`/Game/Outslay/PlayerCharacter/PlayerCharacter.CE_Play Harvest Montage` _asplayer_character "/Game/505_Survival_Mocap_Animations/Animations_UE5/IP/Harvest/IP_Standing_Harvest_Down_Montage.IP_Standing_Harvest_Down_Montage" 1.6 0.0 true))
                  (:`NewEnumerator1`
                    (`/Game/Outslay/PlayerCharacter/PlayerCharacter.CE_Play Harvest Montage` _asplayer_character "/Game/505_Survival_Mocap_Animations/Animations_UE5/IP/Harvest/IP_Standing_Harvest_Mid_Montage.IP_Standing_Harvest_Mid_Montage" 1.6 0.0 true))
                  (:`NewEnumerator2`
                    (`/Game/Outslay/PlayerCharacter/PlayerCharacter.CE_Play Harvest Montage` _asplayer_character "/Game/505_Survival_Mocap_Animations/Animations_UE5/IP/Harvest/IP_Standing_Harvest_Up_Montage.IP_Standing_Harvest_Up_Montage" 1.6 0.0 true))))
              (:`NewEnumerator0`
                (goto _label))
              (:`NewEnumerator1`
                (goto _label))
              (:`NewEnumerator3`
                (switch `/Game/Outslay/Blueprints/Items/Data/E_ItempPos` (`self.Item Location`)
                  (:`NewEnumerator0`
                    (`/Game/Outslay/PlayerCharacter/PlayerCharacter.CE_Play Harvest Montage` _asplayer_character "/Game/505_Survival_Mocap_Animations/Animations_UE5/IP/Harvest/IP_Crouch_Harvest_Mid_Montage.IP_Crouch_Harvest_Mid_Montage" 1.6 0.0 true))
                  (:`NewEnumerator1`
                    (`/Game/Outslay/PlayerCharacter/PlayerCharacter.CE_Play Harvest Montage` _asplayer_character "/Game/505_Survival_Mocap_Animations/Animations_UE5/IP/Harvest/IP_Crouch_Harvest_Mid_Montage.IP_Crouch_Harvest_Mid_Montage" 1.6 0.0 true))
                  (:`NewEnumerator2`
                    (`/Game/Outslay/PlayerCharacter/PlayerCharacter.CE_Play Harvest Montage` _asplayer_character "/Game/505_Survival_Mocap_Animations/Animations_UE5/IP/Harvest/IP_Crouch_Harvest_Up_Montage.IP_Crouch_Harvest_Up_Montage" 1.6 0.0 true))))))))
      (:`then_1`
        (if (!= (`/Game/Outslay/Blueprints/Items/OS_ItemBase.Item Name` (`/Game/Outslay/PlayerCharacter/PlayerCharacter.Get Held Item` _asplayer_character_2)) "Bow")
          (`SceneComponent.SetVisibility` (`/Game/Outslay/PlayerCharacter/PlayerCharacter.ChildActor` _asplayer_character_2) false false))))))

(fn `Get Class`
  (params (Name :type Name))
  (returns (`Item Class` :type "/Game/Outslay/Blueprints/Items/MeleeWeapon/OS_MeleeWeaponBase Class Reference"))
  (switch `name` Name
    (:`Bat`
      (return "/Game/Outslay/Blueprints/Items/MeleeWeapon/Weapons/BP_Bat.BP_Bat_C"))
    (:`Pipe`
      (return "/Game/Outslay/Blueprints/Items/MeleeWeapon/Weapons/BP_Pipe.BP_Pipe_C"))
    (:`Knife`
      (return "/Game/Outslay/Blueprints/Items/MeleeWeapon/Weapons/BP_Knife.BP_Knife_C"))
    (:`Crowbar`
      (return "/Game/Outslay/Blueprints/Items/MeleeWeapon/Weapons/BP_Crowbar.BP_Crowbar_C"))
    (:`Wrench`
      (return "/Game/Outslay/Blueprints/Items/MeleeWeapon/Weapons/BP_Wrench.BP_Wrench_C"))
    (:`Saw`
      (return "/Game/Outslay/Blueprints/Items/MeleeWeapon/Weapons/BP_Saw.BP_Saw_C"))))

(fn `On Held State Change`
  (params (Held :type Boolean))
  (set `/Game/InteractionEssentials/Blueprints/Components/InteractionComponent.bIsActivated` (not Held) (`self.Tap`))
  (set `self.Is Held` Held))

(fn `Should  Wait`
  (returns (ReturnValue :type Boolean))
  (bind (_item _item_type) (`/Game/Outslay/PlayerCharacter/PlayerCharacter.Get Held Item` (`/Game/Outslay/Blueprints/Librarys/OS_FunctionLibrary.Get OS Player Character`)))
  (return (and (select `bool` (== (`/Game/Outslay/Blueprints/Items/OS_ItemBase.Item Name` _item) "Bow") :`false` (select `/Game/Outslay/PlayerCharacter/UI/ItemWheel/Data/E_ItemType` _item_type :`NewEnumerator0` true :`NewEnumerator1` true)) (or (`|EnumEquality` (`self.Item Type`) "NewEnumerator2") (`|EnumEquality` (`self.Item Type`) "NewEnumerator0") (`|EnumEquality` (`self.Item Type`) "NewEnumerator1")))))

(fn `UserConstructionScript`)