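; Thrown explosive projectile for grenades, dynamite and Molotovs, with mesh and behavior chosen by ItemName and Mesh variables.
; It launches along the player's ThrowRef, gradually tilting in flight, with a lit tip effect on non-grenades.
; Molotovs shatter on first bounce into a timed fire effect, while others play throttled bounce sounds and start a fuse.
; Grenade and dynamite share an explosion with radial impulse before delayed self-destruction.
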(event `CE_Activate Tip Effect`
  (params (Activate :type Boolean))
  (bind _niagara (`self.Niagara`))
  (if Activate
    (`ActorComponent.Activate` _niagara true)
    (`ActorComponent.Activate` (`self.Tip Cue`) true)
    (`GameplayStatics.PlaySoundAtLocation` "/Game/The_Sound_Of_Survival_Vol1/CUE/Enviroment/Bonfire/CUE_Place_Bonfire_With_Fire_01_Cue.CUE_Place_Bonfire_With_Fire_01_Cue" (`self.K2_GetActorLocation`) (struct) 1.0 1.0 0.0 null null null null)
    (else
      (`ActorComponent.Deactivate` _niagara)
      (`ActorComponent.Deactivate` (`self.Tip Cue`)))))

(event `self.ReceiveBeginPlay`
  (`|ExecutionSequence`
    (:`then_0`
      (if (!= (`self.Item Name`) "Grenade")
        (`SceneComponent.K2_AttachToComponent` (`self.Niagara`) (`self.StaticMesh`) "Tip" "SnapToTarget" "SnapToTarget" "KeepRelative" true)
        (`self.CE_Activate Tip Effect` true)
        (else
          (`GameplayStatics.PlaySoundAtLocation` "/Game/The_Sound_Of_Survival_Vol1/CUE/Pick_Up_Materials/Pick_Up_Metal_Pieces/CUE_Pick_Up_Metal_Pieces_11_Cue.CUE_Pick_Up_Metal_Pieces_11_Cue" (`self.K2_GetActorLocation`) (struct) 1.0 1.0 0.0 null null null null))))
    (:`then_1`
      (`StaticMeshComponent.SetStaticMesh` (`self.StaticMesh`) (`self.Mesh`))
      (set `MovementComponent.Velocity` (* (`SceneComponent.GetForwardVector` (`/Game/Outslay/PlayerCharacter/PlayerCharacter.ThrowRef` (`/Game/Outslay/Blueprints/Librarys/OS_FunctionLibrary.Get OS Player Character`))) 1000.0) (`self.ProjectileMovement`)))))

(event `self.ReceiveTick`
  (params (DeltaSeconds :type "Float (single-precision)"))
  (bind (_returnvalue_roll _returnvalue_pitch _returnvalue_yaw) (`KismetMathLibrary.BreakRotator` (`self.K2_GetActorRotation`)))
  (bind _returnvalue (`GameplayStatics.GetWorldDeltaSeconds`))
  (`self.K2_SetActorRotation` (`KismetMathLibrary.MakeRotator` (`KismetMathLibrary.FInterpTo` _returnvalue_roll 0.0 _returnvalue 2.0) (`KismetMathLibrary.FInterpTo` _returnvalue_pitch 90.0 _returnvalue 2.0) _returnvalue_yaw)))

(event `self.ProjectileMovement.OnProjectileBounce`
  (params (ImpactResult :type "HitResult Structure (by ref)") (ImpactVelocity :type "Vector Structure (by ref)"))
  (bind _item_name (`self.Item Name`))
  (if (== _item_name "Molotov")
    (`self.CE_Boom`)
    (elif (`SceneComponent.IsVisible` (`self.StaticMesh`))
      (`|ExecutionSequence`
        (:`then_0`
          (`/Engine/EditorBlueprintResources/StandardMacros.DoOnce` false
            (:`Completed`
              (`KismetSystemLibrary.Delay` 2.5)
              (`self.CE_Boom`))))
        (:`then_1`
          (`/Engine/EditorBlueprintResources/StandardMacros.DoOnce` false :!label _label
            (:`Completed`
              (`GameplayStatics.PlaySoundAtLocation` (select `bool` (== _item_name "Dynamite") :`false` "/Game/The_Sound_Of_Survival_Vol1/CUE/Pick_Up_Materials/Pick_Up_Metal_Pieces/CUE_Pick_Up_Metal_Pieces_09_Cue.CUE_Pick_Up_Metal_Pieces_09_Cue" :`true` "/Game/The_Sound_Of_Survival_Vol1/CUE/Inventory/Drop_Wood_From_Inventory/CUE_Drop_Wood_From_Inventory_02_Cue.CUE_Drop_Wood_From_Inventory_02_Cue" :!type "SoundBase Object Reference") (`SceneComponent.K2_GetComponentLocation` (`self.StaticMesh`)) (struct) 1.0 1.0 0.0 null null null null)
              (`KismetSystemLibrary.Delay` 0.36)
              (goto _label :!via `Reset`))))))))

(event `CE_Boom`
  (bind _returnvalue (`self.K2_GetActorLocation`))
  (bind _actor_last_location (`self.Actor Last Location`))
  (bind _actor_last_location_2 (`self.Actor Last Location`))
  (`/Engine/EditorBlueprintResources/StandardMacros.DoOnce` false
    (:`Completed`
      (`self.CE_Activate Tip Effect` false)
      (switch `name` (`self.Item Name`)
        (:`Dynamite`
          (`NiagaraFunctionLibrary.SpawnSystemAtLocation` "/Game/BallisticsVFX/Particles/Explosive/NS_Explosion_GrenadeLauncher_1.NS_Explosion_GrenadeLauncher_1" _returnvalue (struct) (1.0 1.0 1.0) true true "AutoRelease" :!label _label_2)
          (`GameplayStatics.SpawnSoundAtLocation` "/Game/BallisticsVFX/SFX/Explodes/Explosions.Explosions" _returnvalue (struct) 0.75 (`GameplayStatics.GetGlobalTimeDilation`) 0.0 null null)
          (`RadialForceComponent.FireImpulse` (`self.RadialForce`))
          (`SceneComponent.SetVisibility` (`self.StaticMesh`) false true)
          (`KismetSystemLibrary.Delay` 4.0)
          (`self.K2_DestroyActor`))
        (:`Grenade`
          (goto _label_2))
        (:`Molotov`
          (set `self.Actor Last Location` (`self.K2_GetActorLocation`))
          (`GameplayStatics.PlaySoundAtLocation` "/Game/BallisticsVFX/SFX/Impacts/Glass_Impacts.Glass_Impacts" _actor_last_location (struct) 1.0 1.0 0.0 null null null null)
          (`NiagaraFunctionLibrary.SpawnSystemAtLocation` "/Game/BallisticsVFX/Particles/Destruction/Fractures/NS_Fracture_Glass.NS_Fracture_Glass" _actor_last_location (struct) (1.0 1.0 1.0) true true "AutoRelease")
          (`SceneComponent.SetVisibility` (`self.StaticMesh`) false false)
          (`KismetSystemLibrary.Delay` 0.2)
          (bind _returnvalue_2 (`GameplayStatics.SpawnEmitterAtLocation` "/Game/Realistic_Starter_VFX_Pack_Vol2/Particles/Fire/P_Fire_Big.P_Fire_Big" _actor_last_location_2))
          (bind _returnvalue_3 (`GameplayStatics.SpawnSoundAtLocation` "/Game/The_Sound_Of_Survival_Vol1/CUE/Enviroment/Bonfire/CUE_Bonfire_Loop_01_Cue.CUE_Bonfire_Loop_01_Cue" _actor_last_location_2 (struct) 0.75 (`GameplayStatics.GetGlobalTimeDilation`) 0.0 null null))
          (`KismetSystemLibrary.Delay` 6.0)
          (`ActorComponent.Deactivate` _returnvalue_3)
          (`ActorComponent.Deactivate` _returnvalue_2)
          (`self.K2_DestroyActor`))))))

(fn `UserConstructionScript`)