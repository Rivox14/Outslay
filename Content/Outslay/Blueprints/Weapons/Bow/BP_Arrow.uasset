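; BP_Arrow is the bow's arrow projectile, handling what happens when the arrow hits something.
; On impact it spawns a Cubit impact FX spawner with a long decal life, its sounds and VFX switched off, and a fixed impact type regardless of ricochet.
; On blocking hits it also spawns a timed, offset Arrow_Mesh attached to the hit component, so the arrow appears stuck, and plays a random sound there.
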(event `self.ReceiveBeginPlay`)

(event `self.OnImpact`
  (params (Ricochet :type Boolean) (PassedThrough :type Boolean) (Location :type "Vector Structure") (IncomingVelocity :type "Vector Structure") (Normal :type "Vector Structure") (ExitLocation :type "Vector Structure") (ExitVelocity :type "Vector Structure") (Impulse :type "Vector Structure") (PenetrationDepth :type "Float (single-precision)") (Actor :type "Actor Object Reference") (Component :type "SceneComponent Object Reference") (BoneName :type Name) (PhysMaterial :type "PhysicalMaterial Object Reference") (HitResult :type "HitResult Structure"))
  (bind (_bblockinghit _binitialoverlap _time _distance _location _impactpoint _normal _impactnormal _physmat _hitactor _hitcomponent) (`GameplayStatics.BreakHitResult` HitResult))
  (`self.Spawn Impact FX` HitResult IncomingVelocity IncomingVelocity "NewEnumerator2" ExitVelocity)
  (if _bblockinghit
    (bind _returnvalue (`|SpawnActorFromClass` "/Game/Outslay/Blueprints/Weapons/Bow/Arrow_Mesh.Arrow_Mesh_C" (`KismetMathLibrary.MakeTransform` _impactpoint (`self.K2_GetActorRotation`)) "AlwaysSpawn" "OverrideRootScale" null null))
    (`self.SetLifeSpan` _returnvalue 400.0)
    (`self.K2_AttachToComponent` _returnvalue _hitcomponent "None" "KeepWorld" "KeepWorld" "KeepWorld" true)
    (`SceneComponent.K2_SetRelativeLocation` (`/Game/Outslay/Blueprints/Weapons/Bow/Arrow_Mesh.StaticMesh` _returnvalue) (-56.0 0.0 0.0) false false)
    (`GameplayStatics.PlaySoundAtLocation` (`KismetArrayLibrary.Array_Random` (`self.Sound`)) (`self.K2_GetActorLocation` _returnvalue) (struct) 1.0 1.0 0.0 null null null null)))

(event `Spawn Impact FX`
  (params (HitResult :type "HitResult Structure") (RicochetVector :type "Vector Structure") (`Impact Velocity` :type "Vector Structure") (`Impact Type` :type "/Game/BallisticsVFX/FXSpawnerBlueprints/FXSpawners/BPData/ImpactType Enum" :default "NewEnumerator0") (RicochetExitVelocity :type "Vector Structure"))
  (`|SpawnActorFromClass` "/Game/BallisticsVFX/FXSpawnerBlueprints/FXSpawners/Cubit_ImpactFX_Spawner.Cubit_ImpactFX_Spawner_C" (`self.GetTransform` self) "AlwaysSpawn" "MultiplyWithRoot" null HitResult RicochetVector true "NewEnumerator1" false null (`KismetMathLibrary.VSize` `Impact Velocity`) (`KismetMathLibrary.VSize` RicochetExitVelocity) 900.0 "NewEnumerator3" true `Impact Type` false false true "0.000000,0.000000,0.000000|0.000000,0.000000,-0.000000|1.000000,1.000000,1.000000" 0.7 null 500.0 null false false null))

(fn `UserConstructionScript`)