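; Revolver D22 WK weapon Blueprint that exposes eight bullet meshes as external shells.
; GetExternalShellMeshes refills the supplied array with Bullet01 through Bullet08 and returns the count.
; NotifyExternalShellToggle sets the visibility of Bullet01 only, without propagating to its children.
; The construction script only calls its parent, and the BeginPlay, overlap and Tick events are disabled stubs.
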(event `/Game/WeaponKit/Blueprints/Classes/BP_WeaponActorBase_WK.Notify_ExternalShellToggle`
  (params (bOn :type Boolean))
  (`SceneComponent.SetVisibility` (`self.Bullet01`) bOn false))

(fn `GetExternalShellMeshes`
  (params (MeshArray :type "Array of MeshComponent Object Reference (by ref)"))
  (returns (NumMeshes :type Integer))
  (`KismetArrayLibrary.Array_Clear` MeshArray)
  (`KismetArrayLibrary.Array_Add` MeshArray (`self.Bullet01`))
  (`KismetArrayLibrary.Array_Add` MeshArray (`self.Bullet02`))
  (`KismetArrayLibrary.Array_Add` MeshArray (`self.Bullet03`))
  (`KismetArrayLibrary.Array_Add` MeshArray (`self.Bullet04`))
  (`KismetArrayLibrary.Array_Add` MeshArray (`self.Bullet05`))
  (`KismetArrayLibrary.Array_Add` MeshArray (`self.Bullet06`))
  (`KismetArrayLibrary.Array_Add` MeshArray (`self.Bullet07`))
  (bind _returnvalue (`KismetArrayLibrary.Array_Add` MeshArray (`self.Bullet08`)))
  (return (+ _returnvalue 1)))

(fn `UserConstructionScript`
  (`parent.UserConstructionScript`))