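; Base bullet actor for Outslay weapons that drives projectile trail visuals and hands impact effects to a spawner.
; BeginPlay activates the Niagara ricochet trail and shrapnel flame.
; OnImpact overrides the physical material to Water for ocean collision components, then calls SpawnImpactFX.
; That event spawns a Cubit_ImpactFX_Spawner with hit data, speeds and ricochet sound; impact type is fixed, leaving the ricochet-based selection unused.
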(event `self.ReceiveBeginPlay`
  (bind _ns_ricochettrail (`self.NS_RicochetTrail`))
  (`NiagaraComponent.SetAsset` _ns_ricochettrail "/Game/BallisticsVFX/Particles/Impacts/DynamicRicochet/NS_DynamicRicochet_Trail_Generic.NS_DynamicRicochet_Trail_Generic" true)
  (`ActorComponent.Activate` _ns_ricochettrail true)
  (`ActorComponent.Activate` (`self.NS_ShrapnelFlame`) true))

(event `self.OnImpact`
  (params (Ricochet :type Boolean) (PassedThrough :type Boolean) (Location :type "Vector Structure") (IncomingVelocity :type "Vector Structure") (Normal :type "Vector Structure") (ExitLocation :type "Vector Structure") (ExitVelocity :type "Vector Structure") (Impulse :type "Vector Structure") (PenetrationDepth :type "Float (single-precision)") (Actor :type "Actor Object Reference") (Component :type "SceneComponent Object Reference") (BoneName :type Name) (PhysMaterial :type "PhysicalMaterial Object Reference") (HitResult :type "HitResult Structure"))
  (bind (_bblockinghit _binitialoverlap _time _distance _location _impactpoint _normal _impactnormal _physmat _hitactor _hitcomponent _hitbonename _bonename _hititem _elementindex _faceindex _tracestart _traceend) (`GameplayStatics.BreakHitResult` HitResult))
  (`self.Spawn Impact FX` (`GameplayStatics.MakeHitResult` _bblockinghit _binitialoverlap _time _distance _location _impactpoint _normal _impactnormal (select `bool` (`.bSuccess` (cast `OceanBoxCollisionComponent` _hitcomponent :!pure true)) :`false` _physmat :`true` "/Game/BallisticsVFX/PhysMats/Water.Water") _hitactor null _hitbonename _bonename _hititem _elementindex _faceindex _tracestart _traceend) IncomingVelocity IncomingVelocity "NewEnumerator2" ExitVelocity))

(event `Spawn Impact FX`
  (params (HitResult :type "HitResult Structure") (RicochetVector :type "Vector Structure") (`Impact Velocity` :type "Vector Structure") (`Impact Type` :type "/Game/BallisticsVFX/FXSpawnerBlueprints/FXSpawners/BPData/ImpactType Enum" :default "NewEnumerator0") (RicochetExitVelocity :type "Vector Structure"))
  (`|SpawnActorFromClass` "/Game/BallisticsVFX/FXSpawnerBlueprints/FXSpawners/Cubit_ImpactFX_Spawner.Cubit_ImpactFX_Spawner_C" (`self.GetTransform` self) "AlwaysSpawn" "MultiplyWithRoot" null HitResult RicochetVector true "NewEnumerator1" false (`self.RichochetSound`) (`KismetMathLibrary.VSize` `Impact Velocity`) (`KismetMathLibrary.VSize` RicochetExitVelocity) 900.0 "NewEnumerator0" true `Impact Type` false false true "0.000000,0.000000,0.000000|0.000000,0.000000,-0.000000|1.000000,1.000000,1.000000" 0.7 null 500.0 null true true null))

(fn `UserConstructionScript`)