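; Base weapon Blueprint for the player, handling firing, reloading, shell ejection and magazine drop effects.
; Full-auto fire loops on a rate delay into the EBBarrel component, whose ShotFired event decrements ammo and drives sound, muzzle flash, montage and inventory updates.
; Muzzle smoke activates on trigger release to avoid stacking, while bows forward fire calls to BP_Bow.
; Reloads use timed delays, with shotgun duration scaled by round count.
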(event `self.ReceiveTick`
  (params (DeltaSeconds :type "Float (single-precision)")))

(event `self.ReceiveBeginPlay`
  (bind _ebbarrel (`self.EBBarrel`))
  (bind _firerate (`self.FireRate`))
  (`|ExecutionSequence`
    (:`then_0`
      (set `EBBarrel.FireMode` (`self.Fire Mode`) _ebbarrel)
      (bind _bullet_class (`self.Bullet Class`)
        (:`then`
          (`KismetArrayLibrary.Array_Add` (`EBBarrel.Ammo` _ebbarrel) _bullet_class)
          (set `EBBarrel.FireRateMax` _firerate _ebbarrel)
          (set `EBBarrel.FireRateMin` _firerate _ebbarrel))
        (:`else`)))
    (:`then_1`
      (bind _asplayer_character (cast `/Game/Outslay/PlayerCharacter/PlayerCharacter` (`GameplayStatics.GetPlayerCharacter` 0)))
      (set `self.Player Character` _asplayer_character))))

(event `CE_StartFire`
  ;[1 1 1] Fire
  (if (`self.Is Bow`)
    (bind _asbp_bow (cast `/Game/Outslay/Blueprints/Weapons/Bow/BP_Bow` self))
    (`/Game/Outslay/Blueprints/Weapons/Bow/BP_Bow.Bow Ready For Fire` _asbp_bow)
    (else
      (switch `EFireMode` (`self.Fire Mode`)
        (:`FM_Auto`
          _)
        (:`FM_Burst`
          (`/Engine/EditorBlueprintResources/StandardMacros.DoOnce` false :!label _label
            (:`Completed`
              _))))
      (`|ExecutionSequence`
        (:`then_0`
          (if (> (`self.Loaded Ammo`) 0)
            (`EBBarrel.Shoot` (`self.EBBarrel`) true)
            (else
              (set `self.Fire Empty` true)
              (set `self.Fire` false)
              (`/Engine/EditorBlueprintResources/StandardMacros.DoOnce` false :!label _label_2
                (:`Completed`
                  (`self.Fire SFX`)
                  (bind _player_character (`self.Player Character`)
                    (:`then`
                      (`/Game/Outslay/PlayerCharacter/PlayerCharacter.CE_Play Fire Montage` _player_character)
                      (`KismetSystemLibrary.Delay` 1.0)
                      (goto _label_2 :!via `Reset`))
                    (:`else`)))))))
        (:`then_1`
          (goto _label_3 :!via `Reset`))
        (:`then_2`
          (`KismetSystemLibrary.Delay` (/ 1.0 (`self.FireRate`)))
          (goto _label :!via `Reset`))))))

(event `Fire SFX`
  (`GameplayStatics.SpawnSoundAttached` (select `bool` (`self.Fire Empty`) :`false` (`self.Fire Sound`) :`true` (`self.Fire Empty Sound`)) (`self.MuzzelFX`) "None" (0.0 0.0 0.0) (struct) "KeepRelativeOffset" false 1.0 (`GameplayStatics.GetGlobalTimeDilation`) 0.0 null null))

(event `StopFire`
  ;[1 1 1] Fire
  (if (`self.Is Bow`)
    (bind _asbp_bow (cast `/Game/Outslay/Blueprints/Weapons/Bow/BP_Bow` self))
    (`/Game/Outslay/Blueprints/Weapons/Bow/BP_Bow.Bow Fire` _asbp_bow)
    (else
      (`/Engine/EditorBlueprintResources/StandardMacros.DoOnce` true :!label _label_3
        (:`Completed`
          (`EBBarrel.Shoot` (`self.EBBarrel`) false)
          (`self.CE_Trigger On_Off` false)
          (set `self.Fire Empty` false)
          (set `self.Fire` false))))))

(event `CE_Trigger On_Off`
  (params (On :type Boolean))
  (if (`self.Fire Empty`)
    _
    (elif On
      (`self.TriggerON`)
      (else
        (`self.TriggerOFF`)))))

(event `CE_Eject shell`
  (params (EjectForce :type "Float (double-precision)") (EjectRotateForce :type "Float (double-precision)") (Lifetime :type "Float (double-precision)"))
  ;[1 1 1] Eject shell
  (`|SpawnActorFromClass` (`self.Shell Class`) (`SceneComponent.GetSocketTransform` (`self.WeaponMesh`) "ShellEject" "RTS_World") "AlwaysSpawn" "MultiplyWithRoot" null true EjectForce EjectRotateForce Lifetime null (struct :`R` 1.0 :`G` 1.0 :`B` 1.0 :`A` 1.0) null))

(event `MuzzleSmokeOff`
  ;[0.2075 0.4327 1] MUZZLE SMOKE OFF
  (`ActorComponent.Deactivate` (`self.NS_Muzzle_Smoke_light`)))

(event `TriggerON`
  ;[0.2075 0.4327 1] Activate Muzzle Smoke FX once trigger is lifted (we don't want to spawn too many smoke FX during rapid fire)
  (`self.MuzzleSmokeOff`))

(event `TriggerOFF`
  ;[0.2075 0.4327 1] Activate Muzzle Smoke FX once trigger is lifted (we don't want to spawn too many smoke FX during rapid fire)
  (`ActorComponent.Activate` (`self.NS_Muzzle_Smoke_light`) false))

(event `CE_Reload`
  (bind _ammo (`self.Ammo`))
  (bind _mag_size (`self.Mag Size`))
  (bind _returnvalue (* (`KismetMathLibrary.Conv_IntToDouble` (`KismetMathLibrary.SelectInt` _ammo (- _mag_size (`self.Loaded Ammo`)) (< _ammo _mag_size))) 0.67))
  ;[1 1 1] Reload
  (if (not (`self.Is Bow`))
    (`/Engine/EditorBlueprintResources/StandardMacros.DoOnce` false :!label _label_4
      (:`Completed`
        (if (`self.Can Reload`)
          (`|ExecutionSequence`
            (:`then_0`
              (if (== (`self.Weapon Name`) "Shotgun")
                (`KismetSystemLibrary.RetriggerableDelay` 0.4)
                (set `self.Reloading` true)
                (`KismetSystemLibrary.RetriggerableDelay` _returnvalue)
                (else
                  (set `self.Reloading` true)
                  (`KismetSystemLibrary.RetriggerableDelay` 0.5)))
              (if (> (`self.Ammo`) (`self.Mag Size`))
                (set `self.Ammo` (- (`self.Ammo`) (- (`self.Mag Size`) (`self.Loaded Ammo`))))
                (set `self.Loaded Ammo` (`self.Mag Size`))
                (`/Game/Outslay/PlayerCharacter/PlayerCharacter.Update Inventory` (`self.Player Character`))
                (else
                  (set `self.Loaded Ammo` (`self.Ammo`))
                  (set `self.Ammo` 0)
                  (`/Game/Outslay/PlayerCharacter/PlayerCharacter.Update Inventory` (`self.Player Character`)))))
            (:`then_1`
              (if (== (`self.Weapon Name`) "Shotgun")
                (`BlueprintMapLibrary.Map_Add` (`/Game/Outslay/PlayerCharacter/PlayerCharacter.Reload Montages Time` (`self.Player Character`)) "Shotgun" _returnvalue)
                (`KismetSystemLibrary.RetriggerableDelay` _returnvalue)
                (set `self.Reloading` false)
                (else
                  (`KismetSystemLibrary.RetriggerableDelay` 0.2)
                  (set `self.Reloading` false))))
            (:`then_2`
              (`KismetSystemLibrary.RetriggerableDelay` 2.0)
              (goto _label_4 :!via `Reset`))))))))

(event `Play Mag Unload Sound`
  (bind _mag (`self.Mag`))
  ;[1 1 1] Play Mag Sound
  (`GameplayStatics.PlaySoundAtLocation` (`self.Mag Unload SFX`) (`SceneComponent.K2_GetComponentLocation` (`self.Mag`)) (struct) 1.0 1.0 0.0 null null null null)
  (bind _mag_class (`self.Mag Class`)
    (:`then`
      (`|SpawnActorFromClass` _mag_class (`SceneComponent.K2_GetComponentToWorld` _mag) "AdjustIfPossibleButAlwaysSpawn" "MultiplyWithRoot" null false true 60.0 null)
      (`SceneComponent.SetVisibility` _mag false false))
    (:`else`)))

(event `Play Mag Load Sound`
  ;[1 1 1] Play Mag Sound
  (`GameplayStatics.PlaySoundAtLocation` (`self.Mag Load SFX`) (`SceneComponent.K2_GetComponentLocation` (`self.Mag`)) (struct) 1.0 1.0 0.0 null null null null)
  (`SceneComponent.SetVisibility` (`self.Mag`) true false))

(event `self.EBBarrel.ShotFired`
  ;[1 1 1] On Shot Fired
  (if (not (`self.Is Bow`))
    (`|ExecutionSequence`
      (:`then_0`
        (set `self.Fire` true)
        (set `self.Fire Empty` false)
        (`/Engine/EditorBlueprintResources/StandardMacros.DecrementInt` (`self.Loaded Ammo`)
          (:`  `
            (`self.CE_Trigger On_Off` true)
            (`self.Fire SFX`)
            (`self.Activate Muzzel FX`)
            (bind _player_character (`self.Player Character`)
              (:`then`
                (`/Game/Outslay/PlayerCharacter/PlayerCharacter.CE_Play Fire Montage` _player_character)
                (`KismetSystemLibrary.RetriggerableDelay` 0.2)
                (set `self.Fire` false))
              (:`else`)))))
      (:`then_1`
        (`/Game/Outslay/PlayerCharacter/PlayerCharacter.Update Inventory` (`self.Player Character`)))
      (:`then_2`
        (if (<= (`self.Loaded Ammo`) 0)
          (`EBBarrel.Shoot` (`self.EBBarrel`) false)
          (`self.CE_Trigger On_Off` false))))))

(fn `Activate Muzzel FX`
  (bind _muzzelfx (`self.MuzzelFX`))
  (if (not (`self.Fire Empty`))
    (`NiagaraFunctionLibrary.SpawnSystemAttached` "/Game/BallisticsVFX/Particles/Muzzle/MuzzleFlash/NS_Muzzle_Flash_Small.NS_Muzzle_Flash_Small" _muzzelfx "None" (`SceneComponent.GetSocketLocation` _muzzelfx "None") (`Controller.GetControlRotation` (`GameplayStatics.GetPlayerController` 0)) "KeepWorldPosition" true true "AutoRelease")))

(fn `Can Reload`
  (returns (ReturnValue :type Boolean))
  (return (and (< (`self.Loaded Ammo`) (`self.Mag Size`)) (> (`self.Ammo`) 0))))

(fn `UserConstructionScript`
  (`|ExecutionSequence`
    (:`then_0`
      (if (`self.Has Muzzel`)
        (`SceneComponent.SetVisibility` (`self.Muzzel`) true false)
        (`SceneComponent.K2_SetRelativeLocation` (`self.MuzzelFX`) (`KismetMathLibrary.MakeVector` (`self.MuzzelFXlocation`)) false false)
        (else
          (`SceneComponent.SetVisibility` (`self.Muzzel`) false false)
          (`SceneComponent.K2_SetRelativeLocation` (`self.MuzzelFX`) (0.0 0.0 0.0) false false))))))