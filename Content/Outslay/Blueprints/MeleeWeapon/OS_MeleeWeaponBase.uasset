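; Base melee weapon Blueprint that plays combo attack montages on the player character, cached at BeginPlay.
; CE_Attack uses the AttackCombo macro to pick a montage index, then has the player play it slightly sped up.
; The macro rate-limits attacks with DoOnce and Delay, and resets the combo via RetriggerableDelay after inactivity.
; Its counter increments before branching, so from zero it alternates attacks B and C.
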(event `self.ReceiveBeginPlay`
  (bind _asplayer_character (cast `/Game/Outslay/PlayerCharacter/PlayerCharacter` (`GameplayStatics.GetPlayerCharacter` 0)))
  (set `self.Player Character` _asplayer_character))

(event `CE_Attack`
  (bind _output (`|GetArrayItem` (`self.Attack Montages`) (`self.Attack Index`)))
  (`self.Attack Combo` (`self.Attack Gap`)
    (:`Attack A`
      (set `self.Attack Index` 0))
    (:`Attack B`
      (set `self.Attack Index` 1))
    (:`Attack C`
      (set `self.Attack Index` 2)))
  (`/Engine/EditorBlueprintResources/StandardMacros.IsValid` _output
    (:`Is Valid`
      (`/Game/Outslay/PlayerCharacter/PlayerCharacter.CE_Play Attack Montage` (`self.Player Character`) _output 1.2))))

(fn `UserConstructionScript`)