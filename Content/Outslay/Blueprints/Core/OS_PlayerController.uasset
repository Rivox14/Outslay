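; OS_PlayerController is a player controller that tracks which input device the player is using.
; Any key press sets its InputDevice and the menu controller component's CurrentInputDevice, choosing between gamepad and non-gamepad by testing the key.
; PS5 builds skip that test, setting InputDevice to a third value, also applied at BeginPlay, while the menu component gets the gamepad value.
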(event `Key|AnyKey` :consume false :overrideparent false
  (params (Key :type "Key Structure"))
  (bind _bp_menucontrollercomponent (`self.BP_MenuControllerComponent`))
  (:`Pressed`
    (if (`self.PS5 Build`)
      (set `self.Input Device` "NewEnumerator2")
      (set `/Game/MenuSystemPro/Blueprints/Player/BP_MenuControllerComponent.CurrentInputDevice` "NewEnumerator1" (`self.BP_MenuControllerComponent`))
      (elif (`KismetInputLibrary.Key_IsGamepadKey` Key)
        (set `self.Input Device` "NewEnumerator1")
        (set `/Game/MenuSystemPro/Blueprints/Player/BP_MenuControllerComponent.CurrentInputDevice` "NewEnumerator1" _bp_menucontrollercomponent)
        (else
          (set `self.Input Device` "NewEnumerator0")
          (set `/Game/MenuSystemPro/Blueprints/Player/BP_MenuControllerComponent.CurrentInputDevice` "NewEnumerator0" _bp_menucontrollercomponent))))))

(event `self.ReceiveBeginPlay`
  (if (`self.PS5 Build`)
    (set `self.Input Device` "NewEnumerator2")))

(fn `UserConstructionScript`)