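; Player state for Outslay that holds the player's inventory, with separate arrays per item type.
; AddItem stores ranged and melee weapons, using name-based FindItem to detect duplicates; a new melee weapon overwrites the third slot when full.
; UpdateItem writes ammo back for both ranged categories, but its melee durability update is unconnected.
; FindItem also searches throwables, consumables, tools and raw materials, which neither event handles.
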(event `Add Item`
  (params (Item :type "/Game/Outslay/Blueprints/Items/OS_ItemBase Object Reference"))
  (bind ((`RangedWeapons2_49_8EC38D754C37BFF68E9345B3680F8635` _rangedweapons2)) (break `/Game/Outslay/PlayerCharacter/UI/Inventory/Data/S_Inventory_Data` (`self.Inventory`)))
  (bind ((`RangedWeapons_43_01C7ECFC44B590A7C83CD78C0F64D113` _rangedweapons)) (break `/Game/Outslay/PlayerCharacter/UI/Inventory/Data/S_Inventory_Data` (`self.Inventory`)))
  (bind ((`MeleeWeapons_45_12A04DD749A3592FA21E1590EB7AD030` _meleeweapons)) (break `/Game/Outslay/PlayerCharacter/UI/Inventory/Data/S_Inventory_Data` (`self.Inventory`)))
  (switch `/Game/Outslay/PlayerCharacter/UI/ItemWheel/Data/E_ItemType` (`/Game/Outslay/Blueprints/Items/OS_ItemBase.Item Type` Item)
    (:`NewEnumerator0`
      (bind _asos_weapon_base (cast `/Game/Outslay/Blueprints/Items/Weapons/OS_WeaponBase` Item))
      (bind _item_name (`/Game/Outslay/Blueprints/Items/OS_ItemBase.Item Name` _asos_weapon_base))
      (bind (_item_index _found) (`self.Find Item` "NewEnumerator0" _item_name))
      (if _found
        (bind _structout (setmembers `/Game/Outslay/PlayerCharacter/UI/Inventory/Data/S_InventoryWeapon` :`StructRef` (`|GetArrayItem` _rangedweapons _item_index)))
        (`KismetArrayLibrary.Array_Set` _rangedweapons _item_index _structout)
        (else
          (`KismetArrayLibrary.Array_Add` _rangedweapons (make `/Game/Outslay/PlayerCharacter/UI/Inventory/Data/S_InventoryWeapon` _item_name (`/Game/Outslay/Blueprints/Items/Weapons/OS_WeaponBase.Loaded Ammo` _asos_weapon_base) (`/Game/Outslay/Blueprints/Items/Weapons/OS_WeaponBase.Mag Size` _asos_weapon_base) (`/Game/Outslay/Blueprints/Items/Weapons/OS_WeaponBase.Ammo` _asos_weapon_base) true (`/Game/Outslay/Blueprints/Items/Weapons/OS_WeaponBase.Weapon Icon` _asos_weapon_base))))))
    (:`NewEnumerator1`
      (bind _asos_weapon_base_2 (cast `/Game/Outslay/Blueprints/Items/Weapons/OS_WeaponBase` Item))
      (bind _item_name_2 (`/Game/Outslay/Blueprints/Items/OS_ItemBase.Item Name` _asos_weapon_base_2))
      (bind (_item_index_2 _found_2) (`self.Find Item` "NewEnumerator1" _item_name_2))
      (if _found_2
        (bind _structout_2 (setmembers `/Game/Outslay/PlayerCharacter/UI/Inventory/Data/S_InventoryWeapon` :`StructRef` (`|GetArrayItem` _rangedweapons2 _item_index_2)))
        (`KismetArrayLibrary.Array_Set` _rangedweapons2 _item_index_2 _structout_2)
        (else
          (`KismetArrayLibrary.Array_Add` _rangedweapons2 (make `/Game/Outslay/PlayerCharacter/UI/Inventory/Data/S_InventoryWeapon` _item_name_2 (`/Game/Outslay/Blueprints/Items/Weapons/OS_WeaponBase.Loaded Ammo` _asos_weapon_base_2) (`/Game/Outslay/Blueprints/Items/Weapons/OS_WeaponBase.Mag Size` _asos_weapon_base_2) (`/Game/Outslay/Blueprints/Items/Weapons/OS_WeaponBase.Ammo` _asos_weapon_base_2) true (`/Game/Outslay/Blueprints/Items/Weapons/OS_WeaponBase.Weapon Icon` _asos_weapon_base_2))))))
    (:`NewEnumerator2`
      (bind _asos_melee_weapon_base (cast `/Game/Outslay/Blueprints/Items/MeleeWeapon/OS_MeleeWeaponBase` Item))
      (bind _item_name_3 (`/Game/Outslay/Blueprints/Items/OS_ItemBase.Item Name` _asos_melee_weapon_base))
      (bind (_item_index_3 _found_3) (`self.Find Item` "NewEnumerator2" _item_name_3))
      (if _found_3
        (bind _durability (`/Game/Outslay/Blueprints/Items/MeleeWeapon/OS_MeleeWeaponBase.Durability` _asos_melee_weapon_base))
        (bind _structout_3 (setmembers `/Game/Outslay/PlayerCharacter/UI/Inventory/Data/S_InventoryItem` :`StructRef` (`|GetArrayItem` _meleeweapons _item_index_3) :`Durability` _durability))
        (`KismetArrayLibrary.Array_Set` _meleeweapons _item_index_3 _structout_3)
        (elif (>= (`KismetArrayLibrary.Array_Length` _meleeweapons) 3)
          (bind _icon (`/Game/Outslay/Blueprints/Items/MeleeWeapon/OS_MeleeWeaponBase.Icon` _asos_melee_weapon_base))
          (bind _structout_4 (setmembers `/Game/Outslay/PlayerCharacter/UI/Inventory/Data/S_InventoryItem` :`StructRef` (`|GetArrayItem` _meleeweapons 2) :`Name` _item_name_3 :`ItemImage` _icon :`Durability` _durability))
          (`KismetArrayLibrary.Array_Set` _meleeweapons 2 _structout_4)
          (else
            (`KismetArrayLibrary.Array_Add` _meleeweapons (make `/Game/Outslay/PlayerCharacter/UI/Inventory/Data/S_InventoryItem` _item_name_3 1 1 _icon _durability))))))))

(event `Update Item`
  (params (Item :type "/Game/Outslay/Blueprints/Items/OS_ItemBase Object Reference"))
  (bind ((`RangedWeapons_43_01C7ECFC44B590A7C83CD78C0F64D113` _rangedweapons) (`RangedWeapons2_49_8EC38D754C37BFF68E9345B3680F8635` _rangedweapons2)) (break `/Game/Outslay/PlayerCharacter/UI/Inventory/Data/S_Inventory_Data` (`self.Inventory`)))
  (switch `/Game/Outslay/PlayerCharacter/UI/ItemWheel/Data/E_ItemType` (`/Game/Outslay/Blueprints/Items/OS_ItemBase.Item Type` Item)
    (:`NewEnumerator0`
      (bind _asos_weapon_base (cast `/Game/Outslay/Blueprints/Items/Weapons/OS_WeaponBase` Item))
      (for (_array_element _array_index) _rangedweapons
        (if (== (`.Name_2_705CBE8D49FE2139F658798B44ACBAE9` (break `/Game/Outslay/PlayerCharacter/UI/Inventory/Data/S_InventoryWeapon` _array_element)) (`/Game/Outslay/Blueprints/Items/OS_ItemBase.Item Name` _asos_weapon_base))
          (bind _structout (setmembers `/Game/Outslay/PlayerCharacter/UI/Inventory/Data/S_InventoryWeapon` :`StructRef` _array_element :`Loaded Ammo` (`/Game/Outslay/Blueprints/Items/Weapons/OS_WeaponBase.Loaded Ammo` _asos_weapon_base) :`Ammo` (`/Game/Outslay/Blueprints/Items/Weapons/OS_WeaponBase.Ammo` _asos_weapon_base)))
          (`KismetArrayLibrary.Array_Set` _rangedweapons _array_index _structout))))
    (:`NewEnumerator1`
      (bind _asos_weapon_base_2 (cast `/Game/Outslay/Blueprints/Items/Weapons/OS_WeaponBase` Item))
      (for (_array_element_2 _array_index_2) _rangedweapons2
        (if (== (`.Name_2_705CBE8D49FE2139F658798B44ACBAE9` (break `/Game/Outslay/PlayerCharacter/UI/Inventory/Data/S_InventoryWeapon` _array_element_2)) (`/Game/Outslay/Blueprints/Items/OS_ItemBase.Item Name` _asos_weapon_base_2))
          (bind _structout_2 (setmembers `/Game/Outslay/PlayerCharacter/UI/Inventory/Data/S_InventoryWeapon` :`StructRef` _array_element_2 :`Loaded Ammo` (`/Game/Outslay/Blueprints/Items/Weapons/OS_WeaponBase.Loaded Ammo` _asos_weapon_base_2) :`Ammo` (`/Game/Outslay/Blueprints/Items/Weapons/OS_WeaponBase.Ammo` _asos_weapon_base_2)))
          (`KismetArrayLibrary.Array_Set` _rangedweapons2 _array_index_2 _structout_2))))
    (:`NewEnumerator2`
      (bind _asos_melee_weapon_base (cast `/Game/Outslay/Blueprints/Items/MeleeWeapon/OS_MeleeWeaponBase` Item)))))

(fn `Find Item`
  (params (`Item Type` :type "/Game/Outslay/PlayerCharacter/UI/ItemWheel/Data/E_ItemType Enum" :default "NewEnumerator0") (Name :type Name))
  (returns (`Item Index` :type Integer) (Found :type Boolean))
  (bind (_rangedweapons _rangedweapons2 _meleeweapons _throwable _consumables _other _rawmaterials) (break `/Game/Outslay/PlayerCharacter/UI/Inventory/Data/S_Inventory_Data` (`self.Inventory`)))
  (switch `/Game/Outslay/PlayerCharacter/UI/ItemWheel/Data/E_ItemType` `Item Type`
    (:`NewEnumerator0`
      (for (_array_element _array_index) _rangedweapons
        (if (== (`.Name_2_705CBE8D49FE2139F658798B44ACBAE9` (break `/Game/Outslay/PlayerCharacter/UI/Inventory/Data/S_InventoryWeapon` _array_element)) (`local.Name`))
          (return _array_index true)))
      (return 0 false))
    (:`NewEnumerator1`
      (for (_array_element_2 _array_index_2) _rangedweapons2
        (if (== (`.Name_2_705CBE8D49FE2139F658798B44ACBAE9` (break `/Game/Outslay/PlayerCharacter/UI/Inventory/Data/S_InventoryWeapon` _array_element_2)) (`local.Name`))
          (return _array_index_2 true)))
      (return 0 false))
    (:`NewEnumerator2`
      (for (_array_element_3 _array_index_3) _meleeweapons
        (if (== (`.Name_2_705CBE8D49FE2139F658798B44ACBAE9` (break `/Game/Outslay/PlayerCharacter/UI/Inventory/Data/S_InventoryItem` _array_element_3)) (`local.Name`))
          (return _array_index_3 true)))
      (return 0 false))
    (:`NewEnumerator3`
      (for (_array_element_4 _array_index_4) _throwable
        (if (== (`.Name_2_705CBE8D49FE2139F658798B44ACBAE9` (break `/Game/Outslay/PlayerCharacter/UI/Inventory/Data/S_InventoryItem` _array_element_4)) (`local.Name`))
          (return _array_index_4 true)))
      (return 0 false))
    (:`NewEnumerator4`
      (for (_array_element_5 _array_index_5) _consumables
        (if (== (`.Name_2_705CBE8D49FE2139F658798B44ACBAE9` (break `/Game/Outslay/PlayerCharacter/UI/Inventory/Data/S_InventoryItem` _array_element_5)) (`local.Name`))
          (return _array_index_5 true)))
      (return 0 false))
    (:`NewEnumerator5`
      (for (_array_element_6 _array_index_6) _other
        (if (== (`.Name_2_705CBE8D49FE2139F658798B44ACBAE9` (break `/Game/Outslay/PlayerCharacter/UI/Inventory/Data/S_InventoryItem` _array_element_6)) (`local.Name`))
          (return _array_index_6 true)))
      (return 0 false))
    (:`NewEnumerator6`
      (for (_array_element_7 _array_index_7) _rawmaterials
        (if (== (`.Name_2_705CBE8D49FE2139F658798B44ACBAE9` (break `/Game/Outslay/PlayerCharacter/UI/Inventory/Data/S_InventoryItem` _array_element_7)) (`local.Name`))
          (return _array_index_7 true)))
      (return 0 false))))

(fn `UserConstructionScript`)