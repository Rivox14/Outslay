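; BP_Tree is a scatter actor, named for trees, whose construction script lays a row of static mesh components along local Y.
; Count and Distance set the row, and each component gets a random yaw and a mesh from StaticMeshs.
; BrushsData maps meshes to scale ranges for randomized scaling, but its entries come from separate random picks, so an assigned mesh can lack one.
; The event graph is unused.
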(fn `UserConstructionScript`
  (bind _outitem (`KismetArrayLibrary.Array_Random` (`self.Static Meshs`)))
  (for _index (range (`self.Count`))
    (bind _returnvalue (`AddComponent|NODE_AddStaticMeshComponent-0` :`RelativeTransform` (`KismetMathLibrary.MakeTransform` (`KismetMathLibrary.MakeVector` 0.0 (`KismetMathLibrary.Conv_IntToDouble` (* _index (`self.Distance`)))) (`KismetMathLibrary.MakeRotator` 0.0 0.0 (`KismetMathLibrary.RandomFloatInRange` 0.0 360.0)))))
    (`BlueprintMapLibrary.Map_Add` (`self.Brushs Data`) (break `/Game/Outslay/Maps/Bluepints/Data/S_Bush` _outitem) (make `/Game/Outslay/Maps/Bluepints/Data/S_scale` (`.ScaleMin_18_6B4E062C4305BF5F092CF9ADBF400264` (break `/Game/Outslay/Maps/Bluepints/Data/S_Bush` _outitem)) (`.ScaleMax_20_32A9967248456FAC1DFF67AC286DF062` (break `/Game/Outslay/Maps/Bluepints/Data/S_Bush` _outitem))))
    (`StaticMeshComponent.SetStaticMesh` _returnvalue (break `/Game/Outslay/Maps/Bluepints/Data/S_Bush` _outitem))
    (bind _value (`BlueprintMapLibrary.Map_Find` (`self.Brushs Data`) (`StaticMeshComponent.StaticMesh` _returnvalue)))
    (bind _returnvalue_2 (`KismetSystemLibrary.MakeLiteralDouble` (`KismetMathLibrary.RandomFloatInRange` (break `/Game/Outslay/Maps/Bluepints/Data/S_scale` _value) (`.ScaleMax_20_32A9967248456FAC1DFF67AC286DF062` (break `/Game/Outslay/Maps/Bluepints/Data/S_scale` _value)))))
    (`SceneComponent.SetWorldScale3D` _returnvalue (`KismetMathLibrary.MakeVector` _returnvalue_2 _returnvalue_2 _returnvalue_2))))