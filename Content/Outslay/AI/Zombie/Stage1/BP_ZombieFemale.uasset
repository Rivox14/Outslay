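; Female zombie character Blueprint for stage 1 zombie AI that provides visual variants of the enemy.
; The construction script runs the parent's, then switches on the Zombie selector to assign one of several dress, jeans, shorts or girl skeletal meshes to Mesh.
; Zombie 14 reuses the green jeans mesh of Zombie 06.
; The event graph holds only disabled placeholder events, adding no runtime logic of its own.
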(fn `UserConstructionScript`
  (bind _mesh (`self.Mesh`))
  (`parent.UserConstructionScript`)
  (switch `/Game/Outslay/AI/Zombie/Stage1/E_Zombies` (`self.Zombie`)
    (:`NewEnumerator0`
      (set `SkeletalMeshComponent.SkeletalMeshAsset` "/Game/Zombie_Mega_Bundle/Fml_Zombie_Bundle/Fml_Zombie_Dress/Mesh/SK_FML_Zombie_Dress_Black.SK_FML_Zombie_Dress_Black" _mesh))
    (:`NewEnumerator1`
      (set `SkeletalMeshComponent.SkeletalMeshAsset` "/Game/Zombie_Mega_Bundle/Fml_Zombie_Bundle/Fml_Zombie_Dress/Mesh/SK_FML_Zombie_Dress_Orange.SK_FML_Zombie_Dress_Orange" _mesh))
    (:`NewEnumerator2`
      (set `SkeletalMeshComponent.SkeletalMeshAsset` "/Game/Zombie_Mega_Bundle/Fml_Zombie_Bundle/Fml_Zombie_Dress/Mesh/SK_FML_Zombie_Dress_Red.SK_FML_Zombie_Dress_Red" _mesh))
    (:`NewEnumerator3`
      (set `SkeletalMeshComponent.SkeletalMeshAsset` "/Game/Zombie_Mega_Bundle/Fml_Zombie_Bundle/Fml_Zombie_Dress/Mesh/SK_FML_Zombie_Dress_White.SK_FML_Zombie_Dress_White" _mesh))
    (:`NewEnumerator4`
      (set `SkeletalMeshComponent.SkeletalMeshAsset` "/Game/Zombie_Mega_Bundle/Fml_Zombie_Bundle/Fml_Zombie_Jeans/Mesh/SK_FML_Zombie_Jeans_Black.SK_FML_Zombie_Jeans_Black" _mesh))
    (:`NewEnumerator5`
      (set `SkeletalMeshComponent.SkeletalMeshAsset` "/Game/Zombie_Mega_Bundle/Fml_Zombie_Bundle/Fml_Zombie_Jeans/Mesh/SK_FML_Zombie_Jeans_Green.SK_FML_Zombie_Jeans_Green" _mesh))
    (:`NewEnumerator6`
      (set `SkeletalMeshComponent.SkeletalMeshAsset` "/Game/Zombie_Mega_Bundle/Fml_Zombie_Bundle/Fml_Zombie_Jeans/Mesh/SK_FML_Zombie_Jeans_Orange.SK_FML_Zombie_Jeans_Orange" _mesh))
    (:`NewEnumerator7`
      (set `SkeletalMeshComponent.SkeletalMeshAsset` "/Game/Zombie_Mega_Bundle/Fml_Zombie_Bundle/Fml_Zombie_Jeans/Mesh/SK_FML_Zombie_Jeans_Red.SK_FML_Zombie_Jeans_Red" _mesh))
    (:`NewEnumerator8`
      (set `SkeletalMeshComponent.SkeletalMeshAsset` "/Game/Zombie_Mega_Bundle/Fml_Zombie_Bundle/Fml_Zombie_Jeans/Mesh/SK_FML_Zombie_Jeans_White.SK_FML_Zombie_Jeans_White" _mesh))
    (:`NewEnumerator9`
      (set `SkeletalMeshComponent.SkeletalMeshAsset` "/Game/Zombie_Mega_Bundle/Fml_Zombie_Bundle/Fml_Zombie_Shorts/Mesh/SK_Fml_Zombie_Shorts_Black.SK_Fml_Zombie_Shorts_Black" _mesh))
    (:`NewEnumerator11`
      (set `SkeletalMeshComponent.SkeletalMeshAsset` "/Game/Zombie_Mega_Bundle/Fml_Zombie_Bundle/Fml_Zombie_Shorts/Mesh/SK_Fml_Zombie_Shorts_Red.SK_Fml_Zombie_Shorts_Red" _mesh))
    (:`NewEnumerator12`
      (set `SkeletalMeshComponent.SkeletalMeshAsset` "/Game/Zombie_Mega_Bundle/Fml_Zombie_Bundle/Fml_Zombie_Shorts/Mesh/SK_FML_Zombie_Shorts_White.SK_FML_Zombie_Shorts_White" _mesh))
    (:`NewEnumerator13`
      (set `SkeletalMeshComponent.SkeletalMeshAsset` "/Game/ZombiePackV2/ZombieGirl_B/Mesh/SK_ZombieGirl_B.SK_ZombieGirl_B" _mesh))
    (:`NewEnumerator14`
      (set `SkeletalMeshComponent.SkeletalMeshAsset` "/Game/Zombie_Mega_Bundle/Fml_Zombie_Bundle/Fml_Zombie_Jeans/Mesh/SK_FML_Zombie_Jeans_Green.SK_FML_Zombie_Jeans_Green" _mesh))))