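; BP_ZombieMale is a male zombie character for Stage 1 that provides selectable visual variants of the enemy.
; Its Construction Script runs the parent's, then switches on the Zombie variable to assign one of fourteen skeletal meshes to the Mesh component.
; The event graph holds only disabled default events, so any runtime behavior is left to the parent class.
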(fn `UserConstructionScript`
  (bind _mesh (`self.Mesh`))
  (`parent.UserConstructionScript`)
  (switch `/Game/Outslay/AI/Zombie/Stage1/E_Zombies` (`self.Zombie`)
    (:`NewEnumerator0`
      (set `SkeletalMeshComponent.SkeletalMeshAsset` "/Game/Zombie_Mega_Bundle/Zombie_Casual_Bundle/Zombie_Jeans/Mesh/SK_Zombie_Jeans.SK_Zombie_Jeans" _mesh))
    (:`NewEnumerator1`
      (set `SkeletalMeshComponent.SkeletalMeshAsset` "/Game/Zombie_Mega_Bundle/Zombie_Casual_Bundle/Zombie_Shorts/Mesh/SK_Zombie_Shorts.SK_Zombie_Shorts" _mesh))
    (:`NewEnumerator2`
      (set `SkeletalMeshComponent.SkeletalMeshAsset` "/Game/Zombie_Mega_Bundle/Zombie_Classic_Bundle/Zombie_Classic_Suit/Mesh/SK_Zombie_Business_Suit_Color_Variations_Skin.SK_Zombie_Business_Suit_Color_Variations_Skin" _mesh))
    (:`NewEnumerator3`
      (set `SkeletalMeshComponent.SkeletalMeshAsset` "/Game/Zombie_Mega_Bundle/Zombie_Casual_Bundle/Zombie_Jaket/Mesh/SK_Zombie_Jeaket.SK_Zombie_Jeaket" _mesh))
    (:`NewEnumerator4`
      (set `SkeletalMeshComponent.SkeletalMeshAsset` "/Game/Zombie_Mega_Bundle/Zombie_Casual_Bundle/Zombie_Tshirt_Torn/Mesh/SK_Zombie_TshortTorn.SK_Zombie_TshortTorn" _mesh))
    (:`NewEnumerator5`
      (set `SkeletalMeshComponent.SkeletalMeshAsset` "/Game/Zombie_Mega_Bundle/Zombie_Casual_Bundle/Zombie_Jaket/Mesh/SK_Zombie_Jeaket_Hair.SK_Zombie_Jeaket_Hair" _mesh))
    (:`NewEnumerator6`
      (set `SkeletalMeshComponent.SkeletalMeshAsset` "/Game/Zombie_Mega_Bundle/Zombie_Casual_Bundle/Zombie_Tshirt_Torn/Mesh/SK_Zombie_TshortTorn_Cap.SK_Zombie_TshortTorn_Cap" _mesh))
    (:`NewEnumerator7`
      (set `SkeletalMeshComponent.SkeletalMeshAsset` "/Game/Zombie_Mega_Bundle/Zombie_Casual_Bundle/Zombie_Jeans/Mesh/SK_Zombie_Jeans_Hairs.SK_Zombie_Jeans_Hairs" _mesh))
    (:`NewEnumerator8`
      (set `SkeletalMeshComponent.SkeletalMeshAsset` "/Game/Zombie_Mega_Bundle/Zombie_Classic_Bundle/Zombie_Classic_Shirt/Mesh/SK_Zombie_Shirt.SK_Zombie_Shirt" _mesh))
    (:`NewEnumerator9`
      (set `SkeletalMeshComponent.SkeletalMeshAsset` "/Game/Zombie_Mega_Bundle/Zombie_Classic_Bundle/Zombie_Classic_Pants/Mesh/SK_Zombie_Short_Pants.SK_Zombie_Short_Pants" _mesh))
    (:`NewEnumerator11`
      (set `SkeletalMeshComponent.SkeletalMeshAsset` "/Game/Zombie_Mega_Bundle/Zombie_Casual_Bundle/Zombie_Tshirt_Torn/Mesh/SK_Zombie_TshortTorn_Hair.SK_Zombie_TshortTorn_Hair" _mesh))
    (:`NewEnumerator12`
      (set `SkeletalMeshComponent.SkeletalMeshAsset` "/Game/ZombiePackV2/UrbanZombie/Mesh/SK_UrbanZombie_Body_B.SK_UrbanZombie_Body_B" _mesh))
    (:`NewEnumerator13`
      (set `SkeletalMeshComponent.SkeletalMeshAsset` "/Game/ZombiePackV2/OldManZombie/Mesh/SK_OldManZombie.SK_OldManZombie" _mesh))
    (:`NewEnumerator14`
      (set `SkeletalMeshComponent.SkeletalMeshAsset` "/Game/ZombiePackV2/UrbanZombie/Mesh/SK_UrbanZombie_Body_A.SK_UrbanZombie_Body_A" _mesh))))