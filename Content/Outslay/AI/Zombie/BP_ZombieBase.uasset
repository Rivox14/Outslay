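; Base zombie enemy that wraps a BossBehavior component, setting health from its stage Type and starting state from whether a patrol route exists.
; BossBehavior events and velocity checks set flags that SetState resolves by priority, from death down to idle.
; That state picks random sounds and volume for the audio component, which replays after random pauses until death.
; Being hit widens target search radius and forces combat.
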(event `CE_SetState`
  (bind _returnvalue (`KismetMathLibrary.VSize` (`self.GetVelocity`)))
  (`|ExecutionSequence`
    (:`then_0`
      (if (>= _returnvalue 350.0)
        (set `self.Runnig` true)
        (else
          (set `self.Runnig` false)
          (if (> _returnvalue 15.0)
            (set `self.Moving` true)
            (else
              (set `self.Moving` false))))))
    (:`then_1`
      (`self.Set State`))
    (:`then_2`
      (`/Engine/EditorBlueprintResources/StandardMacros.DoOnce` false
        (:`Completed`
          (`self.CE_Play Sound` false))))
    (:`then_3`
      (switch `/Game/Outslay/AI/Zombie/Data/E_ZombieState` (`self.State`)
        (:`NewEnumerator5`
          (if (not (or (`self.Death`) (`self.Attacking`) (`self.Roar`) (`self.Hit`)))
            (`self.CE_Play Sound` false)))))))

(event `SetUp`
  (bind _boss_behavior (`self.Boss Behavior`))
  (bind _boss_behavior_2 (`self.Boss Behavior`))
  (`|ExecutionSequence`
    (:`then_0`
      (switch `/Game/Outslay/AI/Zombie/Data/E_Zombietype` (`self.Type`)
        (:`NewEnumerator0`
          (set `/Game/BossAIToolkit/Blueprints/BPC_Boss_Behavior.MaxHealth` 120.0 _boss_behavior)
          (set `/Game/BossAIToolkit/Blueprints/BPC_Boss_Behavior.Health` 120.0 (`self.Boss Behavior`)))
        (:`NewEnumerator1`
          (set `/Game/BossAIToolkit/Blueprints/BPC_Boss_Behavior.MaxHealth` 240.0 _boss_behavior)
          (set `/Game/BossAIToolkit/Blueprints/BPC_Boss_Behavior.Health` 240.0 (`self.Boss Behavior`)))
        (:`NewEnumerator2`
          (set `/Game/BossAIToolkit/Blueprints/BPC_Boss_Behavior.MaxHealth` 2000.0 _boss_behavior)
          (set `/Game/BossAIToolkit/Blueprints/BPC_Boss_Behavior.Health` 2000.0 (`self.Boss Behavior`)))
        (:`NewEnumerator3`
          (set `/Game/BossAIToolkit/Blueprints/BPC_Boss_Behavior.MaxHealth` 5000.0 _boss_behavior)
          (set `/Game/BossAIToolkit/Blueprints/BPC_Boss_Behavior.Health` 5000.0 (`self.Boss Behavior`)))))
    (:`then_1`
      (bind _patrol_route (`self.Patrol Route`)
        (:`then`
          (set `/Game/BossAIToolkit/Blueprints/BPC_Boss_Behavior.PatrolRoute` _patrol_route _boss_behavior_2)
          (set `/Game/BossAIToolkit/Blueprints/BPC_Boss_Behavior.InitialState` "NewEnumerator2" _boss_behavior_2))
        (:`else`
          (set `/Game/BossAIToolkit/Blueprints/BPC_Boss_Behavior.InitialState` "NewEnumerator1" _boss_behavior_2))))))

(event `self.ReceiveBeginPlay`
  (`parent.ReceiveBeginPlay`)
  (`self.SetUp`)
  (`KismetSystemLibrary.K2_SetTimerDelegate` (`|CreateDelegate` :!event `CE_SetState`) 1.0 true))

(event `self.ReceiveTick`
  (params (DeltaSeconds :type "Float (single-precision)"))
  (`parent.ReceiveTick` DeltaSeconds))

(event `self.Boss Behavior.OnUseAbility`
  (params (AbilityInfo :type "/Game/BossAIToolkit/Blueprints/Structs/F_BossAbility Structure"))
  (`KismetSystemLibrary.RetriggerableDelay` 0.36)
  (set `self.Attacking` true)
  (`self.CE_SetState`)
  (`KismetSystemLibrary.RetriggerableDelay` 0.1)
  (`self.CE_Play Sound` false))

(event `CE_Play Sound`
  (params (Force :type Boolean))
  (bind _audio (`self.Audio`))
  (if Force
    (`AudioComponent.Stop` (`self.Audio`) :!label _label)
    (`AudioComponent.SetSound` _audio (`self.Get Sound`))
    (`AudioComponent.SetVolumeMultiplier` _audio (select `/Game/Outslay/AI/Zombie/Data/E_ZombieState` (`self.State`) :`NewEnumerator0` 0.6 :`NewEnumerator1` 0.7 :`NewEnumerator5` 0.8 :`NewEnumerator2` 1.2 :`NewEnumerator4` 1.2 :`NewEnumerator3` 1.4 :`NewEnumerator6` 1.3 :!type "Float (single-precision)"))
    (`AudioComponent.Play` _audio 0.0)
    (elif (not (`AudioComponent.IsPlaying` (`self.Audio`)))
      (goto _label))))

(event `self.Boss Behavior.OnEndAbility`
  (params (AbilityInfo :type "/Game/BossAIToolkit/Blueprints/Structs/F_BossAbility Structure"))
  (set `self.Attacking` false))

(event `self.Boss Behavior.OnBossDeath`
  (set `self.Death` true)
  (`self.CE_SetState`)
  (`KismetSystemLibrary.RetriggerableDelay` 0.05)
  (`self.CE_Play Sound` true)
  (`KismetSystemLibrary.Delay` 2.0)
  (`AudioComponent.Stop` (`self.Audio`)))

(event `self.Audio.OnAudioFinished`
  (if (not (`self.Death`))
    (`KismetSystemLibrary.RetriggerableDelay` (`KismetMathLibrary.RandomFloatInRange` 1.0 4.0))
    (`self.CE_Play Sound` false)))

(event `self.Boss Behavior.OnCombatStateChange`
  (params (InCombat :type Boolean))
  (bind _idle_montage (`self.Idle Montage`))
  (if InCombat
    (`/Engine/EditorBlueprintResources/StandardMacros.IsValid` _idle_montage
      (:`Is Valid`
        (`self.StopAnimMontage` _idle_montage))
      (:`Is Not Valid`
        _))
    (set `self.Roar` true)
    (`self.CE_SetState`)
    (`KismetSystemLibrary.RetriggerableDelay` 0.05)
    (`self.CE_Play Sound` false)
    (`KismetSystemLibrary.RetriggerableDelay` 2.0)
    (set `self.Roar` false)))

(event `self.Boss Behavior.OnHit`
  (bind _boss_behavior (`self.Boss Behavior`))
  (set `self.Hit` true)
  (`self.CE_SetState`)
  (set `/Game/BossAIToolkit/Blueprints/BPC_Boss_Behavior.TargetSearchRadius` 15000.0 (`self.Boss Behavior`))
  (`/Game/BossAIToolkit/Blueprints/BPC_Boss_Behavior.TryStartCombat` _boss_behavior)
  (`/Game/BossAIToolkit/Blueprints/BPC_Boss_Behavior.SetCombatState` _boss_behavior true)
  (`KismetSystemLibrary.RetriggerableDelay` 0.05)
  (`self.CE_Play Sound` false)
  (`KismetSystemLibrary.RetriggerableDelay` 2.0)
  (set `self.Hit` false))

(event `self.Boss Behavior.OnIdle`
  (set `self.Moving` false)
  (set `self.Runnig` false)
  (`self.CE_SetState`)
  (`KismetSystemLibrary.RetriggerableDelay` 0.1)
  (`self.CE_Play Sound` false))

(event `CE_PlayMontage`
  (params (MontageToPlay :type "AnimMontage Object Reference (by ref)") (PlayRate :type "Float (single-precision)" :default 1.0) (`Is Idle` :type Boolean))
  (if `Is Idle`
    (set `self.Idle Montage` MontageToPlay))
  (`|PlayMontage` (`self.Mesh`) MontageToPlay PlayRate))

(fn `Get Sound`
  (returns (Sound :type "SoundCue Object Reference"))
  (switch `/Game/Outslay/AI/Zombie/Data/E_ZombieState` (`self.State`)
    (:`NewEnumerator0`
      (return (`KismetArrayLibrary.Array_Random` (`self.Idle Sounds`))))
    (:`NewEnumerator1`
      (return (`KismetArrayLibrary.Array_Random` (`self.Moving Sounds`))))
    (:`NewEnumerator5`
      (return (`KismetArrayLibrary.Array_Random` (`self.Runnig Sounds`))))
    (:`NewEnumerator2`
      (return (`KismetArrayLibrary.Array_Random` (`self.Attack Sounds`))))
    (:`NewEnumerator4`
      (return (`KismetArrayLibrary.Array_Random` (`self.Roar Sounds`))))
    (:`NewEnumerator3`
      (return (`KismetArrayLibrary.Array_Random` (`self.Death Sounds`))))
    (:`NewEnumerator6`
      (return (`KismetArrayLibrary.Array_Random` (`self.Hit Sounds`))))))

(fn `GetPriorityScore`
  (params (Querier :type "Actor Object Reference") (IsEnemy :type Boolean))
  (returns (Score :type "Float (double-precision)"))
  (return 0.0))

(fn `Set State`
  (if (`self.Death`)
    (set `self.State` "NewEnumerator3")
    (elif (`self.Hit`)
      (set `self.State` "NewEnumerator6")
      (elif (`self.Roar`)
        (set `self.State` "NewEnumerator4")
        (elif (`self.Attacking`)
          (set `self.State` "NewEnumerator2")
          (elif (`self.Runnig`)
            (set `self.State` "NewEnumerator5")
            (elif (`self.Moving`)
              (set `self.State` "NewEnumerator1")
              (else
                (set `self.State` "NewEnumerator0")))))))))

(fn `UserConstructionScript`
  (`parent.UserConstructionScript`))