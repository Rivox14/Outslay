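; BP_Man_Preview is a construction-script preview actor for the modular CyberMan character and its outfit pieces.
; Head and clothing meshes follow the Body skeleton via leader pose, and Body plays the chosen animation.
; Boolean options toggle the head and each outfit piece.
; Jacket, T-shirt, gloves and pants toggles also set matching Body material opacity parameters, likely masking skin under clothing.
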(fn `SetOutfitsVisability`
  (bind _isgloveson (`self.IsGlovesOn`))
  (bind _ispantson (`self.IsPantsOn`))
  (bind _isjacketon (`self.IsJacketOn`))
  (bind _istshirton (`self.IsTshirtOn`))
  (`|ExecutionSequence`
    (:`then_0`
      (`SceneComponent.SetVisibility` (`self.SKM_CyberMan_Jacket`) _isjacketon false)
      (`MeshComponent.SetScalarParameterValueOnMaterials` (`self.Body`) "JacketOpacity" (`KismetMathLibrary.Conv_BoolToDouble` _isjacketon)))
    (:`then_1`
      (`SceneComponent.SetVisibility` (`self.SKM_CyberMan_T_shirt`) _istshirton false)
      (`MeshComponent.SetScalarParameterValueOnMaterials` (`self.Body`) "TshirtOpacity" (`KismetMathLibrary.Conv_BoolToDouble` _istshirton)))
    (:`then_2`
      (`SceneComponent.SetVisibility` (`self.SKM_CyberMan_Gloves`) _isgloveson false)
      (`MeshComponent.SetScalarParameterValueOnMaterials` (`self.Body`) "GlovesOpacity" (`KismetMathLibrary.Conv_BoolToDouble` _isgloveson)))
    (:`then_3`
      (`SceneComponent.SetVisibility` (`self.SKM_CyberMan_Bag`) (`self.IsBagOn`) false))
    (:`then_4`
      (`SceneComponent.SetVisibility` (`self.SKM_CyberMan_Pants`) _ispantson false)
      (`MeshComponent.SetScalarParameterValueOnMaterials` (`self.Body`) "PantsOpacity" (`KismetMathLibrary.Conv_BoolToDouble` _ispantson)))
    (:`then_5`
      (`SceneComponent.SetVisibility` (`self.SKM_CyberMan_Kneepads`) (`self.IsKneepadsOn`) false))
    (:`then_6`
      (`SceneComponent.SetVisibility` (`self.SKM_CyberMan_Boots`) (`self.IsBootsOn`) false))))

(fn `UserConstructionScript`
  (`SkinnedMeshComponent.SetLeaderPoseComponent` (`self.Head`) (`self.Body`) false false)
  (`SkinnedMeshComponent.SetLeaderPoseComponent` (`self.SKM_CyberMan_Boots`) (`self.Body`) false false)
  (`SkinnedMeshComponent.SetLeaderPoseComponent` (`self.SKM_CyberMan_Bag`) (`self.Body`) false false)
  (`SkinnedMeshComponent.SetLeaderPoseComponent` (`self.SKM_CyberMan_Jacket`) (`self.Body`) false false)
  (`SkinnedMeshComponent.SetLeaderPoseComponent` (`self.SKM_CyberMan_Kneepads`) (`self.Body`) false false)
  (`SkinnedMeshComponent.SetLeaderPoseComponent` (`self.SKM_CyberMan_Pants`) (`self.Body`) false false)
  (`SkinnedMeshComponent.SetLeaderPoseComponent` (`self.SKM_CyberMan_T_shirt`) (`self.Body`) false false)
  (`SkinnedMeshComponent.SetLeaderPoseComponent` (`self.SKM_CyberMan_Gloves`) (`self.Body`) false false)
  (set `SkeletalMeshComponent.AnimationData` (`self.Animation`) (`self.Body`))
  (`|ExecutionSequence`
    (:`then_0`
      (`SceneComponent.SetVisibility` (`self.Head`) (`self.IsHeadVisible`) false))
    (:`then_1`
      (`self.SetOutfitsVisability`))))